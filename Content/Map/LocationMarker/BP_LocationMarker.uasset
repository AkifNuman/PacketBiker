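; Location marker actor that shows its distance in meters from the player on an Icon widget.
; LocMarker starts on BeginPlay and repeats on a looping timer about 30 times a second, pushing the truncated distance to the widget.
; Without a valid player character it measures from every Scooter_BP actor instead, so the last one found sets the label.
; A marker color call exists but is unconnected.
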(event Custom|LocMarker
  (bind _returnvalue (Game|GetPlayerCharacter 0))
  (Utilities|Time|SetTimerbyEvent (delegate Custom|LocMarker) 0.033333 true)
  (Utilities|IsValid _returnvalue
    (:Is%20Valid
      (Class|BPIMarkerWidget|UpdateDistance(Message) (UserInterface|GetUserWidgetObject (Variables|Default|GetIcon)) (Utilities|Text|ToText(String) (Utilities|String|Append (Utilities|String|ToString(Text) (Utilities|Text|ToText(Integer) (Math|Float|Truncate (/ (Math|Vector|Distance(Vector) (Transformation|GetActorLocation _returnvalue) (Transformation|GetActorLocation)) 1e+02)))) "m"))))
    (:Is%20Not%20Valid
      (bind _outactors (Actor|GetAllActorsOfClass "/Game/Vehicles/Motorcycles/Scooter/Scooter_BP.Scooter_BP_C"))
      (for _array_element _outactors
        (Class|BPIMarkerWidget|UpdateDistance(Message) (UserInterface|GetUserWidgetObject (Variables|Default|GetIcon)) (Utilities|Text|ToText(String) (Utilities|String|Append (Utilities|String|ToString(Text) (Utilities|Text|ToText(Integer) (Math|Float|Truncate (/ (Math|Vector|Distance(Vector) (Transformation|GetActorLocation _array_element) (Transformation|GetActorLocation)) 1e+02)))) "m")))))))

(event EventBeginPlay
  (CallFunction|LocMarker))

(fn ConstructionScript)