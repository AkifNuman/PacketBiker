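; Traffic road segment actor that links to straight, right and left successor splines to route AI vehicles through junctions.
; SetNewSpline favors randomly chosen empty exits using vehicle line traces, with highways always continuing straight, while MoveToDestination picks the exit nearest a target.
; Stop functions select priority lanes by turn and drive side, then trace them for conflicting vehicles.
; BeginPlay snaps parking spline starts onto the road.
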(event EventBeginPlay
  ;[1 1 1] Check if there are parking spaces on this spline and if it finds them, move Spline Point 0 on the street line
  (for _array_element (Variables|RefSpline|GetParkingOnThisSpline)
    (Spline|SetLocationatSplinePoint (Variables|/Game/TrafficSystem/BP_ParkingSpot.BP_ParkingSpot_C|GetParkSpline _array_element) 0 (Spline|FindLocationClosesttoWorldLocation (Variables|Default|GetSpline) (Spline|GetLocationatSplinePoint (Variables|/Game/TrafficSystem/BP_ParkingSpot.BP_ParkingSpot_C|GetParkSpline _array_element) 0 "World") "World") "World" true)))

(fn ConstructionScript
  ;[1 1 1] Draw Line to test directions
  ;;[1 0 0] DEBUG ONLY: Connect only for see lines between spline during connection with other spline and use flush for clear all drawn lines
)

(fn SetNewSpline
  (bind _leftspline (Variables|RefSpline|GetLeftSpline))
  (bind _validspline (Variables|Default|GetValidSpline))
  (bind _vehicleonspline (Variables|Default|GetVehicleOnSpline))
  (bind _path (Variables|Default|GetPath))
  (bind _straightspline (Variables|RefSpline|GetStraightSpline))
  (bind _rightspline (Variables|RefSpline|GetRightSpline))
  (bind _returnvalue (Utilities|Array|LastIndex _path))
  (bind _indexofminvalue (Math|Integer|MinOfIntArray _vehicleonspline))
  (bind _returnvalue_2 (Math|Random|RandomIntegerinRange 0 _returnvalue))
  (bind _output (Utilities|Array|Get(acopy) _path _returnvalue_2))
  (if (not (Variables|Default|GetHighSpeedRoad))
    (Utilities|Array|Clear (Variables|Default|GetPath))
    (Utilities|Array|Clear (Variables|Default|GetValidSpline))
    (Utilities|Array|Clear (Variables|Default|GetVehicleOnSpline))
    (Utilities|Array|Clear (Variables|Default|GetDirections))
    (Utilities|IsValid _straightspline
      (:Is%20Valid
        (Utilities|Array|AddUnique (Variables|Default|GetValidSpline) _straightspline)
        (Utilities|Array|AddUnique (Variables|Default|GetDirections) "Straight"))
      (:Is%20Not%20Valid
        _))
    (Utilities|IsValid _rightspline
      (:Is%20Valid
        (Utilities|Array|AddUnique (Variables|Default|GetValidSpline) _rightspline)
        (Utilities|Array|AddUnique (Variables|Default|GetDirections) "Right"))
      (:Is%20Not%20Valid
        _))
    (Utilities|IsValid _leftspline
      (:Is%20Valid
        (Utilities|Array|AddUnique (Variables|Default|GetValidSpline) _leftspline)
        (Utilities|Array|AddUnique (Variables|Default|GetDirections) "Left"))
      (:Is%20Not%20Valid
        _))
    (if (> (Utilities|Array|Length (Variables|Default|GetValidSpline)) 1)
      (for _array_element (Variables|Default|GetValidSpline)
        ;[1 1 1] Check the number of vehicles on the spline, so as not to create traffic
        (bind _outhits (CallFunction|LineTracetoCheckSpline _array_element))
        (Utilities|Array|AddUnique (Variables|Default|GetVehicleOnSpline) (Utilities|Array|Length _outhits)))
      ;[1 1 1] Check the number of vehicles on the spline is less than 1 and add them to "Path" if true
      (for (_array_element_2 _array_index) (Variables|Default|GetVehicleOnSpline)
        (if (< _array_element_2 1)
          (Utilities|Array|AddUnique (Variables|Default|GetPath) _array_index)))
      ;[1 1 1] If "Path" (array) has at least one value, it returns a random street among those available
      (if (Utilities|Array|IsValidIndex (Variables|Default|GetPath))
        (return (Utilities|Array|Get(acopy) (Variables|Default|GetValidSpline) _output) (Utilities|Array|Get(acopy) (Variables|Default|GetDirections) _output))
        (else
          ;[1 1 1] Returns a random road among those available
          (if (Utilities|Array|IsValidIndex _validspline)
            (return (Utilities|Array|Get(acopy) _validspline _indexofminvalue) (Utilities|Array|Get(acopy) (Variables|Default|GetDirections) _indexofminvalue))
            (else
              (return 0 "")))))
      (else
        (return (Utilities|Array|Get(acopy) (Variables|Default|GetValidSpline)) (Utilities|Array|Get(acopy) (Variables|Default|GetDirections)))))
    (else
      ;[1 1 1] only for Highway
      (return (Variables|RefSpline|GetStraightSpline) "Straight"))))

(fn MovetoDestination
  (params (Location :type Vector))
  (bind _distancetodestination (Variables|Default|GetDIstanceToDestination))
  (bind _straightspline (Variables|RefSpline|GetStraightSpline))
  (bind _rightspline (Variables|RefSpline|GetRightSpline))
  (bind _leftspline (Variables|RefSpline|GetLeftSpline))
  (bind _indexofminvalue (Math|Float|MinOfFloatArray _distancetodestination))
  (Utilities|Array|Clear (Variables|Default|GetDIstanceToDestination))
  (Utilities|Array|Clear (Variables|Default|GetValidSpline))
  (Utilities|Array|Clear (Variables|Default|GetDirections))
  (Utilities|IsValid _straightspline
    (:Is%20Valid
      (Utilities|Array|AddUnique (Variables|Default|GetValidSpline) _straightspline)
      (Utilities|Array|AddUnique (Variables|Default|GetDirections) "Straight"))
    (:Is%20Not%20Valid
      _))
  (Utilities|IsValid _rightspline
    (:Is%20Valid
      (Utilities|Array|AddUnique (Variables|Default|GetValidSpline) _rightspline)
      (Utilities|Array|AddUnique (Variables|Default|GetDirections) "Right"))
    (:Is%20Not%20Valid
      _))
  (Utilities|IsValid _leftspline
    (:Is%20Valid
      (Utilities|Array|AddUnique (Variables|Default|GetValidSpline) _leftspline)
      (Utilities|Array|AddUnique (Variables|Default|GetDirections) "Left"))
    (:Is%20Not%20Valid
      _))
  (for _array_element (Variables|Default|GetValidSpline)
    ;[1 1 1] Check the distance to your destination among the available roads, to use the fastest one
    (Utilities|Array|AddUnique (Variables|Default|GetDIstanceToDestination) (Math|Vector|VectorLength (- (Transformation|GetActorLocation _array_element) Location))))
  ;[1 1 1] Returns the spline closest to the target
  (return (Utilities|Array|Get(acopy) (Variables|Default|GetValidSpline) _indexofminvalue) (Utilities|Array|Get(acopy) (Variables|Default|GetDirections) _indexofminvalue)))

(fn LineTracetoCheckSpline
  (params (Spline :type BP%20Spline%20Road%20Object%20Reference))
  (bind _arrow (Variables|BP_SplineRoad_C|GetArrow Spline))
  (bind _returnvalue (Spline|GetLocationatSplinePoint (Variables|BP_SplineRoad_C|GetSpline Spline) 1 "World"))
  (bind _returnvalue_2 (Spline|GetLocationatSplinePoint (Variables|BP_SplineRoad_C|GetSpline Spline) 0 "World"))
  (bind _returnvalue_3 (Transformation|GetWorldRotation _arrow))
  (bind _returnvalue_4 (Math|Vector|GetForwardVector _returnvalue_3))
  (bind _returnvalue_5 (+ _returnvalue_2 "0, 0,40.000000"))
  ;[1 1 1] Use LineTrace to check the number of vehicles on the spline
  (bind _outhits (Class|KismetSystemLibrary|LineTraceMultiforObjects (+ (* _returnvalue_4 -3.5e+02) _returnvalue_5) (select (< (Math|Vector|VectorLength (- _returnvalue_2 _returnvalue)) 2e+03) (+ _returnvalue "0, 0,40.000000") (+ (* _returnvalue_4 2e+03) _returnvalue_5)) (Utilities|Array|MakeArray "ObjectTypeQuery5") false 0 "None" true))
  (return _outhits))

(fn StopSystemSplineCheck
  (params (VehicleDirection :type String))
  (bind _prioritystraight (Variables|StopSystem|GetPriorityStraight))
  (bind _priorityright (Variables|StopSystem|GetPriorityRight))
  (bind _priorityleft (Variables|StopSystem|GetPriorityLeft))
  (bind _priorityleft_2 (Variables|StopSystem|GetPriorityLeft))
  (bind _priorityleft_3 (Variables|StopSystem|GetPriorityLeft))
  (bind _priorityright_2 (Variables|StopSystem|GetPriorityRight))
  (bind _priorityleft_4 (Variables|StopSystem|GetPriorityLeft))
  (bind _priorityright_3 (Variables|StopSystem|GetPriorityRight))
  (bind _priorityright_4 (Variables|StopSystem|GetPriorityRight))
  (Variables|Default|SetDirection VehicleDirection)
  (Utilities|Map|Clear (Variables|Default|GetSplineStopCheck))
  (switch string (Variables|StopSystem|GetDriveLane)
    (:Right
      (switch string (Variables|Default|GetDirection)
        (:Straight
          (Utilities|IsValid _priorityleft_3
            (:Is%20Valid
              (Utilities|Map|Add (Variables|Default|GetSplineStopCheck) 1 _priorityleft_3))
            (:Is%20Not%20Valid
              _))
          (Utilities|IsValid _priorityright_3
            (:Is%20Valid
              (Utilities|Map|Add (Variables|Default|GetSplineStopCheck) 2 _priorityright_3))
            (:Is%20Not%20Valid
              _)))
        (:Right
          (Utilities|IsValid _priorityleft_2
            (:Is%20Valid
              (Utilities|Map|Add (Variables|Default|GetSplineStopCheck) 1 _priorityleft_2))
            (:Is%20Not%20Valid
              _)))
        (:Left
          (Utilities|IsValid _priorityleft_4 :!label _label
            (:Is%20Valid
              (Utilities|Map|Add (Variables|Default|GetSplineStopCheck) 1 _priorityleft_4))
            (:Is%20Not%20Valid
              _))
          (Utilities|IsValid _prioritystraight
            (:Is%20Valid
              (Utilities|Map|Add (Variables|Default|GetSplineStopCheck) 0 _prioritystraight))
            (:Is%20Not%20Valid
              _))
          (Utilities|IsValid _priorityright_4
            (:Is%20Valid
              (Utilities|Map|Add (Variables|Default|GetSplineStopCheck) 2 _priorityright_4))
            (:Is%20Not%20Valid
              _)))))
    (:Left
      (switch string (Variables|Default|GetDirection)
        (:Straight
          (Utilities|IsValid _priorityleft
            (:Is%20Valid
              (Utilities|Map|Add (Variables|Default|GetSplineStopCheck) 1 _priorityleft))
            (:Is%20Not%20Valid
              _))
          (Utilities|IsValid _priorityright
            (:Is%20Valid
              (Utilities|Map|Add (Variables|Default|GetSplineStopCheck) 2 _priorityright))
            (:Is%20Not%20Valid
              _)))
        (:Right
          (goto _label))
        (:Left
          (Utilities|IsValid _priorityright_2
            (:Is%20Valid
              (Utilities|Map|Add (Variables|Default|GetSplineStopCheck) 2 _priorityright_2))
            (:Is%20Not%20Valid
              _))))))
  (return))

(fn StopSystemVehicleCheck
  (bind _splinestopcheck (Variables|Default|GetSplineStopCheck))
  (bind _keys (Utilities|Map|Keys _splinestopcheck))
  (for _array_element _keys
    (LocalVariables|SetLocIntDirection _array_element)
    (bind (_outhit _returnvalue) (Collision|LineTraceForObjects (+ (* (Math|Vector|GetForwardVector (Variables|BP_SplineRoad_C|GetSpline (.Value (Utilities|Map|Find _splinestopcheck _array_element)))) -4.5e+02) (+ (Spline|GetLocationatSplinePoint (Variables|BP_SplineRoad_C|GetSpline (.Value (Utilities|Map|Find _splinestopcheck _array_element))) (- (Spline|GetNumberOfSplinePoints (Variables|BP_SplineRoad_C|GetSpline (.Value (Utilities|Map|Find _splinestopcheck _array_element)))) 1) "World") "0, 0,40.000000")) (+ (* (Math|Vector|GetForwardVector (Variables|BP_SplineRoad_C|GetSpline (.Value (Utilities|Map|Find _splinestopcheck _array_element)))) (select (== (LocalVariables|GetLocIntDirection) 0) 8e+02 5.5e+02)) (+ (Spline|GetLocationatSplinePoint (Variables|BP_SplineRoad_C|GetSpline (.Value (Utilities|Map|Find _splinestopcheck _array_element))) (- (Spline|GetNumberOfSplinePoints (Variables|BP_SplineRoad_C|GetSpline (.Value (Utilities|Map|Find _splinestopcheck _array_element)))) 1) "World") "0, 0,40.000000")) (Utilities|Array|MakeArray "ObjectTypeQuery5") false 0 "ForDuration" true "(R=0.000000,G=0.000000,B=1.000000,A=1.000000)"))
    (if _returnvalue
      (bind _output_get (LocalVariables|SetVehicleOnSplineCheck (.AsBP%20Base%20Vehicle%20Parent (Utilities|Casting|CastToBP_BaseVehicleParent (.HitActor (Collision|BreakHitResult _outhit))))))
      (if (Variables|BP_SplineRoad_C|GetStopSystem (Variables|/Game/TrafficSystem/BP_BaseVehicleParent.BP_BaseVehicleParent_C|GetOldPath _output_get))
        (if (and (Utilities|Enum|NotEqual(Enum) (Variables|Default|GetDirection) "Right") (not (<= (Default|SpeedtoKMh (LocalVariables|GetVehicleOnSplineCheck)) 1.0)))
          (LocalVariables|SetLocHit true))
        (elif (Utilities|IsValid (Variables|BP_SplineRoad_C|GetRef_TrafficLight (Variables|/Game/TrafficSystem/BP_BaseVehicleParent.BP_BaseVehicleParent_C|GetOldPath _output_get)))
          (if (not (<= (Default|SpeedtoKMh (LocalVariables|GetVehicleOnSplineCheck)) 1.0))
            (LocalVariables|SetLocHit true :!label _label))
          (else
            (goto _label))))))
  (return (LocalVariables|GetLocHit)))