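; Traffic trigger that makes AI vehicles check for oncoming traffic when entering a highway.
; On the server, an overlapping vehicle starts a looping timer that runs CheckVehicle, cleared when an overlap ends.
; Each check line-traces for vehicles along the NextRoad spline, from behind to ahead of the point closest to the entering vehicle.
; A detected vehicle sets Hit on the entering vehicle's BP_AIVehicleController.
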(event OnComponentBeginOverlap(CollisionComponent)
  (params (OverlappedComponent :type Primitive%20Component%20Object%20Reference) (OtherActor :type Actor%20Object%20Reference) (OtherComp :type Primitive%20Component%20Object%20Reference) (OtherBodyIndex :type Integer) (bFromSweep :type Boolean) (SweepResult :type Hit%20Result%20Structure%20%28by%20ref%29))
  (Networking|SwitchHasAuthority
    (:Authority
      (bind _asbp_base_vehicle_parent (Utilities|Casting|CastToBP_BaseVehicleParent OtherActor))
      (Variables|Default|SetRef_Vehicle _asbp_base_vehicle_parent)
      (bind _returnvalue (Utilities|Time|SetTimerbyFunctionName 0 "CheckVehicle" 0.1 true))
      (Variables|Default|SetTimer _returnvalue))))

(event OnComponentEndOverlap(CollisionComponent)
  (params (OverlappedComponent :type Primitive%20Component%20Object%20Reference) (OtherActor :type Actor%20Object%20Reference) (OtherComp :type Primitive%20Component%20Object%20Reference) (OtherBodyIndex :type Integer))
  (Networking|SwitchHasAuthority
    (:Authority
      (Utilities|Time|ClearandInvalidateTimerbyHandle (Variables|Default|GetTimer)))))

(event Custom|CheckVehicle
  (bind _ref_vehicle (Variables|Default|GetRef_Vehicle))
  (bind _nextroad (Variables|Default|GetNextRoad))
  (bind _returnvalue (Transformation|GetActorLocation _ref_vehicle))
  (bind _spline (Variables|/Game/TrafficSystem/BP_SplineRoad.BP_SplineRoad_C|GetSpline _nextroad))
  (bind _returnvalue_2 (Spline|FindLocationClosesttoWorldLocation _spline _returnvalue "World"))
  (bind _returnvalue_3 (Math|Vector|GetForwardVector _spline))
  (bind _returnvalue_4 (+ _returnvalue_2 "0, 0,40.000000"))
  ;[1 1 1] use LineTrace to check that there are no vehicles on the highway
  (bind _returnvalue_5 (Collision|LineTraceForObjects (+ _returnvalue_4 (* _returnvalue_3 -4e+03)) (+ (* _returnvalue_3 1.5e+03) _returnvalue_4) (Utilities|Array|MakeArray "ObjectTypeQuery5") false 0 "ForOneFrame"))
  (if _returnvalue_5
    (Variables|/Game/TrafficSystem/BP_AiVehicleController.BP_AIVehicleController_C|SetHit? (.AsBP%20AIVehicle%20Controller (Utilities|Casting|CastToBP_AIVehicleController (AI|GetAIController (Variables|Default|GetRef_Vehicle)))) true)))

(fn ConstructionScript)