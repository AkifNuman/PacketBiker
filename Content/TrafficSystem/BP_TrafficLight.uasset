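; Replicated traffic light actor that cycles between green, yellow and red.
; On the authority it registers with its referenced light controller, which can trigger green or red changes, or runs its own looping delay-based cycle if none is valid.
; LightNum's RepNotify moves and recolors a single point light to show each state.
; It also disables the box collision on green and turns on query collision at yellow, which carries into red.
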(event Custom|TrafficLightSwitch
  ;[1 1 1] Without Traffic Controller
  (if (Variables|Default|GetCanGo?)
    (Utilities|FlowControl|Delay 6.0)
    (Variables|Default|SetLightNum 0)
    (else
      (Variables|Default|SetLightNum 1)
      (Utilities|FlowControl|Delay 2.0)
      (Variables|Default|SetLightNum 2)))
  (Utilities|FlowControl|Delay 2e+01)
  (Variables|Default|SetCanGo? (not (Variables|Default|GetCanGo?)))
  (CallFunction|TrafficLightSwitch))

(event Custom|Controller%20SetRedLight
  ;[1 1 1] With Traffic Controller
  (Variables|Default|SetLightNum 1)
  (Utilities|FlowControl|Delay 2.0)
  (Variables|Default|SetLightNum 2))

(event Custom|ControllerSetGreenLight
  ;[1 1 1] With Traffic Controller
  (Utilities|FlowControl|Delay 6.0)
  (Variables|Default|SetLightNum 0))

(event EventBeginPlay
  (bind _ref_lightcontroller (Variables|TrafficController|GetRef_LightController))
  ;[1 1 1] Begin Play
  (Networking|SwitchHasAuthority
    (:Authority
      (Utilities|IsValid _ref_lightcontroller
        (:Is%20Valid
          (Utilities|Array|AddUnique (Variables|/Game/TrafficSystem/BP_TrafficLightController.BP_TrafficLightController_C|GetRef_TrafficLight _ref_lightcontroller) self))
        (:Is%20Not%20Valid
          (CallFunction|TrafficLightSwitch))))))

(fn ConstructionScript)

(fn OnRepLightNum
  (bind _pointlight (Variables|Default|GetPointLight))
  (bind _pointlight_2 (Variables|Default|GetPointLight))
  (bind _pointlight_3 (Variables|Default|GetPointLight))
  (bind _relativelocation (Variables|/Script/Engine.SceneComponent|GetRelativeLocation _pointlight_3))
  (bind _relativelocation_2 (Variables|/Script/Engine.SceneComponent|GetRelativeLocation _pointlight))
  (bind _relativelocation_3 (Variables|/Script/Engine.SceneComponent|GetRelativeLocation _pointlight_2))
  (switch int (Variables|Default|GetLightNum)
    (:0
      (Transformation|SetRelativeLocation _pointlight (Math|Vector|MakeVector (.x _relativelocation_2) (.y _relativelocation_2) 1.2e+02) false true)
      (Rendering|Components|Light|SetLightColor (Variables|Default|GetPointLight) "(R=0.010183,G=1.000000,B=0.000000,A=1.000000)" true)
      (Collision|SetCollisionEnabled (Variables|Default|GetBox) "NoCollision"))
    (:1
      (Collision|SetCollisionEnabled (Variables|Default|GetBox) "QueryOnly")
      (Transformation|SetRelativeLocation _pointlight_2 (Math|Vector|MakeVector (.x _relativelocation_3) (.y _relativelocation_3) 134.0) false true)
      (Rendering|Components|Light|SetLightColor (Variables|Default|GetPointLight) "(R=0.958214,G=1.000000,B=0.000000,A=1.000000)" true))
    (:2
      (Transformation|SetRelativeLocation _pointlight_3 (Math|Vector|MakeVector (.x _relativelocation) (.y _relativelocation) 151.0) false true)
      (Rendering|Components|Light|SetLightColor (Variables|Default|GetPointLight) "(R=1.000000,G=0.007234,B=0.000000,A=1.000000)" true))))