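; BP_TriggerHighwayExit is a traffic system trigger that randomly diverts vehicles onto a highway exit path.
; On server-side overlap, a BP_BaseVehicleParent has a one-in-two chance of being sent ChangeLane with NewPath, if that path is valid.
; A DoOnce gate, consumed before the vehicle cast, blocks further overlaps until any end overlap on the server resets it.
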(event OnComponentBeginOverlap(CollisionComponent)
  (params (OverlappedComponent :type Primitive%20Component%20Object%20Reference) (OtherActor :type Actor%20Object%20Reference) (OtherComp :type Primitive%20Component%20Object%20Reference) (OtherBodyIndex :type Integer) (bFromSweep :type Boolean) (SweepResult :type Hit%20Result%20Structure%20%28by%20ref%29))
  (bind _newpath (Variables|Default|GetNewPath))
  (Networking|SwitchHasAuthority
    (:Authority
      (Utilities|FlowControl|DoOnce false
        (:Completed
          (bind _asbp_base_vehicle_parent (Utilities|Casting|CastToBP_BaseVehicleParent OtherActor))
          (if (<= (Math|Random|RandomInteger 6) 2)
            (Utilities|IsValid _newpath
              (:Is%20Valid
                (Default|ChangeLane _asbp_base_vehicle_parent _newpath)))))))))

(event OnComponentEndOverlap(CollisionComponent)
  (params (OverlappedComponent :type Primitive%20Component%20Object%20Reference) (OtherActor :type Actor%20Object%20Reference) (OtherComp :type Primitive%20Component%20Object%20Reference) (OtherBodyIndex :type Integer))
  (bind _newpath (Variables|Default|GetNewPath))
  (Networking|SwitchHasAuthority
    (:Authority
      (Utilities|FlowControl|DoOnce false) ; enters at Reset
    )))

(fn ConstructionScript)