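; BP_TrafficLightController cycles groups of traffic lights so that one group at a time shows green.
; On the server, after a short delay, BeginPlay sorts the TrafficLight map's integer keys in ascending order by repeated minimum extraction.
; A looping timer then calls TrafficLightSwitch, which sets lights that can go to red, turns the next group green and updates their CanGo flags, wrapping around after the last group.
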(event EventBeginPlay
  (bind _trafficlight (Variables|Default|GetTrafficLight))
  (bind _returnvalue (Utilities|Map|Length _trafficlight))
  ;[1 1 1] Begin play
  (Networking|SwitchHasAuthority
    (:Authority
      (Utilities|FlowControl|Delay 0.5)
      (if (> _returnvalue 0)
        (Variables|Default|SetTrafficLightNum _returnvalue)
        (bind _keys (Utilities|Map|Keys (Variables|Default|GetTrafficLight)))
        (Variables|Default|SetKeyList _keys)
        (while (> (Utilities|Array|Length (Variables|Default|GetKeyList)) 0)
          (Utilities|Array|AddUnique (Variables|Default|GetOrderedKeyList) (.MinValue (Math|Integer|MinOfIntArray (Variables|Default|GetKeyList))))
          (Utilities|Array|RemoveIndex (Variables|Default|GetKeyList) (.IndexOfMinValue (Math|Integer|MinOfIntArray (Variables|Default|GetKeyList)))))
        (Utilities|Time|SetTimerbyFunctionName 0 "TrafficLightSwitch" (Variables|Default|GetTimeBetweenLightSwitch) true)))))

(fn ConstructionScript)

(fn TrafficLightSwitch
  (bind _trafficlight (Variables|Default|GetTrafficLight))
  ;[1 1 1] Loop for switching on the traffic lights in the established order
  (bind _keys (Utilities|Map|Keys _trafficlight))
  (for _array_element _keys
    (for _array_element_2 (.trafficlight (.Value (Utilities|Map|Find _trafficlight _array_element)))
      (if (Variables|/Game/TrafficSystem/BP_TrafficLight.BP_TrafficLight_C|GetCanGo? _array_element_2)
        (Default|ControllerSetRedLight _array_element_2)
        (Variables|/Game/TrafficSystem/BP_TrafficLight.BP_TrafficLight_C|SetCanGo? _array_element_2 false))))
  (for _array_element_3 (.trafficlight (.Value (Utilities|Map|Find (Variables|Default|GetTrafficLight) (Utilities|Array|Get(acopy) (Variables|Default|GetOrderedKeyList) (Variables|Default|GetTemp_Num)))))
    (Default|ControllerSetGreenLight _array_element_3)
    (Variables|/Game/TrafficSystem/BP_TrafficLight.BP_TrafficLight_C|SetCanGo? _array_element_3 true))
  (if (== (+ (Variables|Default|GetTemp_Num) 1) (Variables|Default|GetTrafficLightNum))
    (Variables|Default|SetTemp_Num 0)
    (else
      (Variables|Default|SetTemp_Num (+ (Variables|Default|GetTemp_Num) 1)))))