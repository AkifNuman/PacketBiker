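; BP_TargetPoint is a mission destination that completes the mission when the player character or a Scooter_BP overlaps it.
; It checks scooters only when no player character is valid, and requires a BP_TargetCalculator's TarLoc to match its TargetNumber.
; Completion removes the location marker, calculators, counters and mission counter widget, and adds money to Bp_LevelDatabase.
; Cleanup runs as nested GetAllActorsOfClass loops, so the reward repeats per calculator destroyed.
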(event Collision|EventActorBeginOverlap
  (params (OtherActor :type Actor%20Object%20Reference))
  (bind _returnvalue (Game|GetPlayerCharacter 0))
  (Utilities|IsValid _returnvalue
    (:Is%20Valid
      (if (or (== _returnvalue OtherActor) (== OtherActor (stale _array_element_6))) :!label _label
        (bind _outactors (Actor|GetAllActorsOfClass "/Game/Mission/BP_TargetCalculator.BP_TargetCalculator_C"))
        (for _array_element _outactors
          (if (== (Variables|/Game/Mission/BP_TargetCalculator.BP_TargetCalculator_C|GetTarLoc _array_element) (Variables|Default|GetTarget%20Number))
            (bind _returnvalue_2 (Actor|GetActorOfClass "/Game/Map/LocationMarker/BP_LocationMarker.BP_LocationMarker_C"))
            (Actor|DestroyActor _returnvalue_2)
            (bind _outactors_2 (Actor|GetAllActorsOfClass "/Game/Mission/BP_TargetCalculator.BP_TargetCalculator_C"))
            (for _array_element_2 _outactors_2
              (Actor|DestroyActor _array_element_2)
              (bind _outactors_3 (Actor|GetAllActorsOfClass "/Game/Level_Database/BP_LevelDatabase.Bp_LevelDatabase_C"))
              (for _array_element_3 _outactors_3
                (bind _output_get (Variables|/Game/Level_Database/BP_LevelDatabase.Bp_LevelDatabase_C|SetDolar _array_element_3 (+ (Variables|/Game/Level_Database/BP_LevelDatabase.Bp_LevelDatabase_C|GetDolar _array_element_3) 5)))
                (Development|PrintString (Utilities|String|Append (Utilities|String|ToString(Integer) _output_get) "dolar "))
                (bind _outactors_4 (Actor|GetAllActorsOfClass "/Game/Level_Database/BP_Counter.BP_Counter_C"))
                (for _array_element_4 _outactors_4
                  (Actor|DestroyActor _array_element_4)
                  (bind _foundwidgets (Widget|GetAllWidgetsOfClass "/Game/Level_Database/WB_MissionCounter.WB_MissionCounter_C" true))
                  (for _array_element_5 _foundwidgets
                    (Widget|RemovefromParent _array_element_5)))))))))
    (:Is%20Not%20Valid
      (bind _outactors_5 (Actor|GetAllActorsOfClass "/Game/Vehicles/Motorcycles/Scooter/Scooter_BP.Scooter_BP_C"))
      (for _array_element_6 _outactors_5
        (goto _label)))))

(fn ConstructionScript)