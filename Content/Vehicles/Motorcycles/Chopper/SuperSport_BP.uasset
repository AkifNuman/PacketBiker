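; SuperSport_BP is a two-wheeler child Blueprint with flip recovery, timeline-driven lean and steering, and per-character special abilities.
; Ability events trigger DoOnce-and-delay cooldown graphs: Grandma toggles post-process, Grandpa slows time, Samurai boosts, RichFemSciFi teleports forward.
; Cel-shader post-process blendables style the abilities, while dynamic dissolve materials hide the vehicle and rider during teleports.
; A Wizard boost with steam exists, but its event is empty.
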(event Custom|RichFemSci-Fi_AbilityScooter
  (Utilities|RichFemSci-Fi))

(event Custom|GrandmaAbility
  (Utilities|Grandma))

(event Custom|SamuraiAbility
  (Utilities|Samurai))

(event Custom|MakeRevisible
  (bind _movemesh (Variables|Default|GetMoveMesh))
  (bind _dissolveflot (Timeline|Dissolving Reverse)
    (:Update
      (Rendering|Material|SetScalarParameterValueonMaterials _movemesh "Dissolve" _dissolveflot)
      (Rendering|Material|SetScalarParameterValueonMaterials _movemesh "Dissolve" _dissolveflot)
      (Rendering|Material|SetScalarParameterValueonMaterials (Variables|Default|GetCharacter) "Dissolve" _dissolveflot))))

(event Custom|DiasableMovement
  (bind _skeletalmesh (Variables|Default|GetSkeletalMesh))
  (Class|PrimitiveComponent|SetConstraintMode _skeletalmesh "XYPlane")
  (Class|PrimitiveComponent|SetConstraintMode _skeletalmesh "XYPlane"))

(event Custom|WizzardAbility)

(event Custom|MakeUnVisible
  (bind _movemesh (Variables|Default|GetMoveMesh))
  (bind _dissolveflot (Timeline|Dissolving Play)
    (:Update
      (Rendering|Material|SetScalarParameterValueonMaterials _movemesh "Dissolve" _dissolveflot)
      (Rendering|Material|SetScalarParameterValueonMaterials _movemesh "Dissolve" _dissolveflot)
      (Rendering|Material|SetScalarParameterValueonMaterials (Variables|Default|GetCharacter) "Dissolve" _dissolveflot))))

(event Custom|GrandmaDefaultVi)

(event Custom|GrandpaAbility
  (Utilities|Grandpa))

(event Input|ActionEvents|InputActionSteerRight
  (params (Key :type Key%20Structure :default "None"))
  ;[1 1 1 1 113] Scooter
  (:Pressed
    (bind _rightlean (Timeline|Timeline_0_0 Play)
      (:Update
        (Transformation|SetRelativeRotation (Variables|Default|GetMoveMesh) (Math|Rotator|Lerp(Rotator) "0, 0, 0" (Variables|Animations(forShow)|GetEndRotationRight_0) _rightlean) false false)
        (Transformation|SetRelativeRotation (Variables|Default|GetSteer) (Math|Rotator|Lerp(Rotator) "0, 0, 0" (Variables|Animations(forShow)|GetSteerRotationRightEnd_0) _rightlean) false false))))
  (:Released
    (Timeline|Timeline_0_0 Reverse)))

(event Input|ActionEvents|InputActionSteerLeft
  (params (Key :type Key%20Structure :default "None"))
  ;[1 1 1 1 113] Scooter
  (:Pressed
    (Development|PrintString "Left")
    (bind _leftlean (Timeline|Timeline_1 Play)
      (:Update
        (Transformation|SetRelativeRotation (Variables|Default|GetMoveMesh) (Math|Rotator|Lerp(Rotator) "0, 0, 0" (Variables|Animations(forShow)|GetEndRotationLeft_0) _leftlean) false false)
        (Transformation|SetRelativeRotation (Variables|Default|GetSteer) (Math|Rotator|Lerp(Rotator) "0, 0, 0" (Variables|Animations(forShow)|GetSteerRotationLeftEnd_0) _leftlean) false false))))
  (:Released
    (Timeline|Timeline_1 Reverse)))

(event Input|KeyboardEvents|SpaceBar
  (params (Key :type Key%20Structure :default "None"))
  (:Pressed
    (CallFunction|CarFlip)))

(fn ConstructionScript
  (|CallParentFunction))