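; Naked motorcycle vehicle Blueprint that adds steering input on top of its parent class.
; Left and right steer actions set SteerDirectionSct and drive two timelines that rotate the Steer component toward each side's end rotation, reversing on release.
; Space Bar calls CarFlip, and a separate custom event sets the XY-plane constraint mode on MoveMesh and SkeletalMesh.
; The construction script only runs the parent's.
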(event Custom|CustomEvent
  (Class|PrimitiveComponent|SetConstraintMode (Variables|Default|GetMoveMesh) "XYPlane")
  (Class|PrimitiveComponent|SetConstraintMode (Variables|Default|GetSkeletalMesh) "XYPlane"))

(event Input|ActionEvents|InputActionSteerRight
  (params (Key :type Key%20Structure :default "None"))
  (:Pressed
    (Variables|Default|SetSteerDirection_Sct 5e+01)
    (bind _leanright (Timeline|Timeline_0 Play)
      (:Update
        (Transformation|SetRelativeRotation (Variables|Default|GetSteer) (Math|Rotator|Lerp(Rotator) "0, 0, 0" (Variables|Default|GetSteerRotationRightEnd_Sct) _leanright) false false))))
  (:Released
    (Variables|Default|SetSteerDirection_Sct 0.0)
    (Timeline|Timeline_0 Reverse)))

(event Input|ActionEvents|InputActionSteerLeft
  (params (Key :type Key%20Structure :default "None"))
  (:Pressed
    (Variables|Default|SetSteerDirection_Sct -5e+01)
    (bind _leanleft (Timeline|Timeline_1 Play)
      (:Update
        (Transformation|SetRelativeRotation (Variables|Default|GetSteer) (Math|Rotator|Lerp(Rotator) "0, 0, 0" (Variables|Default|GetSteerRotationLeftEnd_Sct) _leanleft) false false))))
  (:Released
    (Variables|Default|SetSteerDirection_Sct 0.0)
    (Timeline|Timeline_1 Reverse)))

(event Input|KeyboardEvents|SpaceBar
  (params (Key :type Key%20Structure :default "None"))
  (:Pressed
    (CallFunction|CarFlip)))

(fn ConstructionScript
  (|CallParentFunction))