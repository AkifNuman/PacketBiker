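; Base drivable motorcycle: player characters mount it via a mesh and anim swap, drive it, and dismount by repossession.
; LeftShift triggers per-character abilities, mostly through a Scooter_BP cast, with dash and slow-motion graphs here.
; Looping timers drain fuel, showing WB_Win when empty, and aim an arrow at location markers.
; Hitting vehicles at speed ejects and ragdolls non-Demon riders; a timeline drives dissolve fades.
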(event OnComponentEndOverlap(Box)
  (params (OverlappedComponent :type Primitive%20Component%20Object%20Reference) (OtherActor :type Actor%20Object%20Reference) (OtherComp :type Primitive%20Component%20Object%20Reference) (OtherBodyIndex :type Integer))
  (Utilities|FlowControl|Delay 1e+01)
  (Utilities|FlowControl|DoOnce false) ; enters at Reset
)

(event OnComponentBeginOverlap(Box)
  (params (OverlappedComponent :type Primitive%20Component%20Object%20Reference) (OtherActor :type Actor%20Object%20Reference) (OtherComp :type Primitive%20Component%20Object%20Reference) (OtherBodyIndex :type Integer) (bFromSweep :type Boolean) (SweepResult :type Hit%20Result%20Structure%20%28by%20ref%29))
  (bind _returnvalue (Utilities|GetClass OtherActor))
  (Utilities|FlowControl|DoOnce false
    (:Completed
      (if (Variables|Default|GetInVehicle)
        (if (not (Variables|Default|GetIsDemon))
          (if (or (or (== _returnvalue "/Game/TrafficSystem/BP_BaseVehicleParent.BP_BaseVehicleParent_C") (== _returnvalue 0)) (or (== _returnvalue "/Game/TrafficSystem/BP_Ferrari_AI.BP_Ferrari_AI_C") (== _returnvalue "/Game/TrafficSystem/BP_PoliceCar_AI.BP_PoliceCar_AI_C")))
            (if (> (Class|WheeledVehicleMovementComponent|GetForwardSpeed (Variables|Default|GetVehicleComponent)) 7.5e+02)
              (CallFunction|OutOfVehicle)
              (bind _asbp_character (Utilities|Casting|CastToBP_Character (Game|Player|GetPlayerPawn 0)))
              (Default|Ragdoll _asbp_character)
              (else
                (Camera|PlayWorldCameraShake "/Game/Characters/MainCharacters/CameraShake/SetupCamShake.SetupCamShake_C" (Transformation|GetWorldLocation (Variables|Default|GetMoveMesh)) 0.0 1.5e+03)))))))))

(event OnComponentEndOverlap(EnterBox)
  (params (OverlappedComponent :type Primitive%20Component%20Object%20Reference) (OtherActor :type Actor%20Object%20Reference) (OtherComp :type Primitive%20Component%20Object%20Reference) (OtherBodyIndex :type Integer))
  (bind _asbp_character (Utilities|Casting|CastToBP_Character OtherActor))
  (Variables|/Game/Characters/BP_Character.BP_Character_C|SetInBox _asbp_character false)
  (Widget|RemovefromParent (stale OnComponentBeginOverlap(EnterBox) _returnvalue)))

(event OnComponentBeginOverlap(EnterBox)
  (params (OverlappedComponent :type Primitive%20Component%20Object%20Reference) (OtherActor :type Actor%20Object%20Reference) (OtherComp :type Primitive%20Component%20Object%20Reference) (OtherBodyIndex :type Integer) (bFromSweep :type Boolean) (SweepResult :type Hit%20Result%20Structure%20%28by%20ref%29))
  (bind _asbp_character (Utilities|Casting|CastToBP_Character OtherActor))
  (Variables|/Game/Characters/BP_Character.BP_Character_C|SetInBox _asbp_character true)
  (bind _returnvalue (UserInterface|CreateWidget "/Game/Interfaces/Basbana.Basbana_C"))
  (UserInterface|Viewport|AddtoViewport _returnvalue 0))

(event Custom|Fueller
  (bind _vehiclecomponent (Variables|Default|GetVehicleComponent))
  (bind _returnvalue (Class|WheeledVehicleMovementComponent|GetForwardSpeed _vehiclecomponent))
  (bind _returnvalue_2 (Math|Float|Truncate _returnvalue))
  (Utilities|Time|SetTimerbyEvent (delegate Custom|Fueller) 0.016667 true)
  (Utilities|IsValid (Game|GetPlayerCharacter 0)
    (:Is%20Not%20Valid
      (if (>= _returnvalue_2 0)
        (Variables|Default|SetFuel (- (Variables|Default|GetFuel) (/ (Math|Conversions|ToFloat(Integer) (+ _returnvalue_2 10)) 1e+04)))
        (if (<= (Variables|Default|GetFuel) 0.0)
          (Variables|Default|SetFuel 0.0)
          (Components|Activation|Deactivate (Variables|Default|GetVehicleComponent))
          (Utilities|FlowControl|DoOnce false
            (:Completed
              (bind _returnvalue_3 (UserInterface|CreateWidget "/Game/Fuel/WB_Win.WB_Win_C"))
              (UserInterface|Viewport|AddtoViewport _returnvalue_3 0))))
        (else
          (Variables|Default|SetFuel (- (Variables|Default|GetFuel) (/ (Math|Conversions|ToFloat(Integer) (+ 0 10)) 2e+03)))
          (if (<= (Variables|Default|GetFuel) 0.0)
            (Variables|Default|SetFuel 0.0)
            (Components|Activation|Deactivate (Variables|Default|GetVehicleComponent))
            (Utilities|FlowControl|DoOnce false
              (:Completed
                (bind _returnvalue_4 (UserInterface|CreateWidget "/Game/Fuel/WB_Win.WB_Win_C"))
                (UserInterface|Viewport|AddtoViewport _returnvalue_4 0)))))))))

(event Custom|PP
  (params (Target :type Post%20Process%20Volume%20Object%20Reference) (InBlendableObject :type Blendable%20Interface%20Interface) (InWeight :type Float%20%28single-precision%29))
  (Rendering|AddorUpdateBlendable Target InBlendableObject InWeight :!class /Script/Engine.PostProcessVolume))

(event Custom|MyThrottle
  (params (Throttle :type Float%20%28single-precision%29)))

(event Custom|MakeUnVisible
  (bind _movemesh (Variables|Default|GetMoveMesh))
  (bind _dissolveflot (Timeline|Timeline_2 Play)
    (:Update
      (Rendering|Material|SetScalarParameterValueonMaterials _movemesh "Dissolve" _dissolveflot)
      (Rendering|Material|SetScalarParameterValueonMaterials _movemesh "Dissolve" _dissolveflot)
      (Rendering|Material|SetScalarParameterValueonMaterials (Variables|Default|GetCharacter) "Dissolve" _dissolveflot))))

(event Custom|MakeRevisible
  (bind _movemesh (Variables|Default|GetMoveMesh))
  (bind _dissolveflot (Timeline|Timeline_2 Reverse)
    (:Update
      (Rendering|Material|SetScalarParameterValueonMaterials _movemesh "Dissolve" _dissolveflot)
      (Rendering|Material|SetScalarParameterValueonMaterials _movemesh "Dissolve" _dissolveflot)
      (Rendering|Material|SetScalarParameterValueonMaterials (Variables|Default|GetCharacter) "Dissolve" _dissolveflot))))

(event Custom|DiasableMovement
  (Class|PrimitiveComponent|SetConstraintMode (Variables|Default|GetMoveMesh) "XYPlane")
  (Class|PrimitiveComponent|SetConstraintMode (Variables|Default|GetSkeletalMesh) "XYPlane"))

(event Custom|ThrottleCustom
  (params (Throttle :type Float%20%28single-precision%29))
  (bind _vehiclecomponent (Variables|Default|GetVehicleComponent))
  ;[1 1 1] BaseControl
  (Class|WheeledVehicleMovementComponent|SetThrottleInput _vehiclecomponent Throttle)
  (Variables|Default|SetSpeed (Class|WheeledVehicleMovementComponent|GetForwardSpeed _vehiclecomponent)))

(event Custom|SteerCustom
  (params (Steering :type Float%20%28single-precision%29))
  ;[1 1 1] BaseControl
  (Class|WheeledVehicleMovementComponent|SetSteeringInput (Variables|Default|GetVehicleComponent) Steering))

(event Custom|GetInVehicle
  (params (InputMesh :type Skeletal%20Mesh%20Object%20Reference) (AnimInstance :type Object%20Class%20Reference) (Character :type Character%20Object%20Reference) (AnimInstanceAfterVehicle :type Object%20Class%20Reference) (IsSamurai :type Boolean) (IsGrandma :type Boolean) (IsWizard :type Boolean) (IsGamerGirl :type Boolean) (IsDemon :type Boolean) (IsGrandpa :type Boolean) (IsHomelessMan :type Boolean) (IsRichFemSci-Fi :type Boolean))
  (Development|PrintString (Utilities|GetDisplayName Character))
  (Variables|Default|SetChar Character)
  (Utilities|WhichCharacter IsSamurai IsGrandma IsWizard IsGamerGirl IsDemon IsGrandpa IsHomelessMan IsRichFemSci-Fi)
  (Variables|Default|SetCharacterAnimClass AnimInstanceAfterVehicle)
  (Rendering|SetVisibility (Variables|Default|GetCharacter) true false)
  (CallFunction|ActivateMovement)
  (Variables|Default|SetInVehicle true)
  (Class|SkinnedMeshComponent|SetSkeletalMesh (Variables|Default|GetCharacter) InputMesh true)
  (Class|SkeletalMeshComponent|SetAnimClass (Variables|Default|GetCharacter) AnimInstance)
  (if (Variables|Default|GetIsWizard)
    (Transformation|SetRelativeLocation (Variables|Default|GetCharacter) "0, 0, 0" false false)
    (Rendering|SetVisibility (Variables|Default|GetStaticMesh) true false)))

(event Custom|ZeroFuel
  (bind _foundwidgets (Widget|GetAllWidgetsOfClass "/Game/Fuel/WB_Win.WB_Win_C" true))
  (Widget|RemovefromParent _foundwidgets)
  (if (!= (Variables|Default|GetDolar2) 0)
    (Utilities|FlowControl|DoOnce false) ; enters at Reset
  ))

(event Custom|arrow2%20set%20directions
  (bind _arrow (Variables|Default|GetArrow))
  (Utilities|Time|SetTimerbyEvent (delegate Custom|arrow2%20set%20directions) 0.033333 true)
  (bind _outactors (Actor|GetAllActorsOfClass 0))
  (if (Utilities|Array|IsValidIndex _outactors)
    (bind _outactors_2 (Actor|GetAllActorsOfClass "/Game/Map/LocationMarker/BP_LocationMarkerRes.BP_LocationMarkerRes_C"))
    (for _array_element _outactors_2
      (Development|SetHiddeninGame _arrow false false)
      (Transformation|SetWorldRotation _arrow (Math|Rotator|FindLookatRotation (Transformation|GetWorldLocation _arrow) (Transformation|GetActorLocation _array_element)) false false))
    (else
      (Development|SetHiddeninGame (Variables|Default|GetArrow) true false))))

(event Custom|DisableExhaust
  (params (Condition :type Boolean) (Target :type Actor%20Component%20Object%20Reference))
  (Utilities|FlowControl|Delay 0.4)
  (if Condition
    (Components|Activation|Deactivate Target)
    (else
      (Components|Activation|Activate Target false))))

(event Custom|OutOfVehicle
  (CallFunction|OutOfVehicleFunc)
  (CallFunction|PP (Variables|Default|GetPostProcess) 0 0.9)
  (Rendering|SetVisibility (Variables|Default|GetStaticMesh) false false)
  (CallFunction|DiasableMovement))

(event EventBeginPlay
  (Utilities|FlowControl|Sequence
    (:then_0
      (bind _returnvalue (UserInterface|CreateWidget "/Game/Vehicles/Speed.Speed_C"))
      (UserInterface|Viewport|AddtoViewport _returnvalue 0)
      (CallFunction|Fueller))
    (:then_1
      (bind _outactors (Actor|GetAllActorsOfClass "/Game/Level_Database/BP_LevelDatabase.Bp_LevelDatabase_C"))
      (for _array_element _outactors
        (Variables|Default|SetDolar2 (Variables|/Game/Level_Database/BP_LevelDatabase.Bp_LevelDatabase_C|GetDolar _array_element))))
    (:then_2
      (CallFunction|Arrow2SetDirections))))

(event EventTick
  (params (DeltaSeconds :type Float%20%28single-precision%29)))

(event Input|AxisEvents|InputAxisThrottle
  (params (AxisValue :type Float%20%28single-precision%29))
  (bind _plane1 (Variables|Default|GetPlane1))
  (bind _particlesystem (Variables|Default|GetParticleSystem))
  ;[1 1 1] BaseControl
  (CallFunction|ThrottleCustom AxisValue)
  (if (> AxisValue 0.0)
    (Components|Activation|Deactivate _particlesystem)
    (elif (< AxisValue 0.0)
      (if (> (Class|WheeledVehicleMovementComponent|GetForwardSpeed (Variables|Default|GetVehicleComponent)) 0.0)
        (Game|SpawnActorfromClass "/Game/Characters/CharacterAbilities/TireTrack/BP_TrackTire.BP_TrackTire_C" (Math|Transform|MakeTransform (Transformation|GetWorldLocation _plane1) (Transformation|GetWorldRotation _plane1) "0.500000,0.500000,0.500000") "AlwaysSpawn" 0 0)
        (Components|Activation|Activate _particlesystem false :!label _label))
      (else
        (goto _label)))))

(event Input|AxisEvents|InputAxisSteer
  (params (AxisValue :type Float%20%28single-precision%29))
  ;[1 1 1] BaseControl
  (CallFunction|SteerCustom AxisValue))

(event Input|KeyboardEvents|1
  (params (Key :type Key%20Structure :default "None")))

(event Input|KeyboardEvents|LeftShift
  (params (Key :type Key%20Structure :default "None"))
  (:Pressed
    (if (Variables|Default|GetIsWizard)
      (bind _asscooter_bp (Utilities|CastScooter))
      (Default|WizzardAbility _asscooter_bp)
      (elif (Variables|Default|GetIsSamurai)
        (bind _asscooter_bp_2 (Utilities|CastScooter))
        (Default|SamuraiAbility _asscooter_bp_2)
        (elif (Variables|Default|GetIsGrandma)
          (bind _outactors (Actor|GetAllActorsOfClass "/Game/Characters/BP_Grandma.BP_Grandma_C"))
          (for _array_element _outactors
            (Default|SpecialForceGrandma _array_element))
          (elif (Variables|Default|GetIsGrandpa)
            (bind _asscooter_bp_3 (Utilities|CastScooter))
            (Default|GrandpaAbility _asscooter_bp_3)
            (elif (Variables|Default|GetIsRichFemSci-Fi)
              (bind _asscooter_bp_4 (Utilities|CastScooter))
              (Default|RichFemSci-FiAbilityScooter _asscooter_bp_4))))))))

(event Input|KeyboardEvents|T
  (params (Key :type Key%20Structure :default "None"))
  (:Pressed
    (CallFunction|OutOfVehicle)))

(fn ConstructionScript
  (|CallParentFunction))

(fn ActivateMovement
  (Class|PrimitiveComponent|SetConstraintMode (Variables|Default|GetMoveMesh) "None")
  (Class|PrimitiveComponent|SetConstraintMode (Variables|Default|GetSkeletalMesh) "None"))

(fn CarFlip
  (bind _returnvalue (Transformation|GetActorRotation))
  (bind _returnvalue_2 (Transformation|GetActorLocation))
  (if (< (Math|Vector|VectorLength (Transformation|GetVelocity)) 2e+01)
    (bind _returnvalue_3 (Transformation|Teleport (+ _returnvalue_2 "0, 0,100.000000") (Math|Rotator|MakeRotator 0.0 0.0 (.yaw _returnvalue))))
    (if _returnvalue_3
      (Development|PrintString "Flipliyo Abi")
      (else
        (Development|PrintString "Senden bi sikim olmaz amk")
        (bind _returnvalue_4 (Transformation|Teleport (+ _returnvalue_2 "0, 0,200.000000") (Math|Rotator|MakeRotator 0.0 0.0 (.yaw _returnvalue))))
        (if (not _returnvalue_4)
          (Development|PrintString "Ben olmasam naneyi yemistin biliyon demi")
          (Transformation|Teleport (+ _returnvalue_2 "100.000000, 0,100.000000") (Math|Rotator|MakeRotator 0.0 0.0 (.yaw _returnvalue))))))))

(fn OutOfVehicleFunc
  (CallFunction|ActivateMovement)
  (Variables|Default|SetInVehicle false)
  (bind _outactors (Actor|GetAllActorsOfClass "/Game/Characters/BP_Character.BP_Character_C"))
  (for _array_element _outactors
    (Rendering|SetVisibility (Variables|/Script/Engine.Character|GetMesh _array_element) true false)
    (Collision|SetActorEnableCollision _array_element true)
    (Transformation|Teleport _array_element (Transformation|GetWorldLocation (Variables|Default|GetOutOf)) "0, 0, 0")
    (Utilities|IsValid _array_element
      (:Is%20Valid
        (Pawn|Possess (Game|GetPlayerController 0) _array_element)
        (Class|SkinnedMeshComponent|SetSkeletalMesh (Variables|Default|GetCharacter) 0 true)))))

(fn MySteer
  (params (Steering1 :type Float%20%28single-precision%29)))