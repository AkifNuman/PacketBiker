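; BP_Scooter is a scooter Blueprint that animates steering lean and detects characters standing near it.
; SteerLeft and SteerRight inputs play timelines that roll MoveMesh and yaw SteerMesh, reversing on release; the LeanRigh and LeanLeft timeline names are swapped relative to direction.
; Box overlaps toggle InBox on BP_Character, with a debug print on entry.
; It contains no driving logic, and its cached samurai pawn reference is unused.
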(event OnComponentBeginOverlap(Box)
  (params (OverlappedComponent :type Primitive%20Component%20Object%20Reference) (OtherActor :type Actor%20Object%20Reference) (OtherComp :type Primitive%20Component%20Object%20Reference) (OtherBodyIndex :type Integer) (bFromSweep :type Boolean) (SweepResult :type Hit%20Result%20Structure%20%28by%20ref%29))
  (bind _asbp_character (Utilities|Casting|CastToBP_Character OtherActor))
  (Variables|/Game/Characters/BP_Character.BP_Character_C|SetInBox _asbp_character true)
  (Development|PrintString "Hello"))

(event OnComponentEndOverlap(Box)
  (params (OverlappedComponent :type Primitive%20Component%20Object%20Reference) (OtherActor :type Actor%20Object%20Reference) (OtherComp :type Primitive%20Component%20Object%20Reference) (OtherBodyIndex :type Integer))
  (bind _asbp_character (Utilities|Casting|CastToBP_Character OtherActor))
  (Variables|/Game/Characters/BP_Character.BP_Character_C|SetInBox _asbp_character false))

(event Custom|charevent
  (params (Charreferance :type Character%20Object%20Reference))
  (Variables|Default|SetCHARACTERIM Charreferance))

(event EventTick
  (params (DeltaSeconds :type Float%20%28single-precision%29)))

(event EventBeginPlay
  (bind _asbp_samurai_warior (Utilities|Casting|CastToBP_SamuraiWarior (Game|Player|GetPlayerPawn 0)))
  (Variables|Default|SetChar _asbp_samurai_warior))

(event Input|ActionEvents|InputActionSteerLeft
  (params (Key :type Key%20Structure :default "None"))
  (:Pressed
    (bind _leftlean (Timeline|LeanRigh Play)
      (:Update
        (Transformation|SetRelativeRotation (Variables|Default|GetMoveMesh) (Math|Rotator|Lerp(Rotator) "0, 0, 0" "0, 0,-15.000000" _leftlean) false false)
        (Transformation|SetRelativeRotation (Variables|Default|GetSteerMesh) (Math|Rotator|Lerp(Rotator) "0, 0, 0" "0,-20.000000, 0" _leftlean) false false))))
  (:Released
    (Timeline|LeanRigh Reverse)))

(event Input|ActionEvents|InputActionSteerRight
  (params (Key :type Key%20Structure :default "None"))
  (:Pressed
    (bind _rightlean (Timeline|LeanLeft Play)
      (:Update
        (Transformation|SetRelativeRotation (Variables|Default|GetMoveMesh) (Math|Rotator|Lerp(Rotator) "0, 0, 0" "0, 0,15.000000" _rightlean) false false)
        (Transformation|SetRelativeRotation (Variables|Default|GetSteerMesh) (Math|Rotator|Lerp(Rotator) "0, 0, 0" "0,20.000000, 0" _rightlean) false false))))
  (:Released
    (Timeline|LeanLeft Reverse)))

(fn ConstructionScript)