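; Drivable scooter Blueprint that takes on the boarding character's mesh, animation and type flags.
; Throttle and steering feed the VehicleComponent, timelines lean body and handlebars, and looping timers drain fuel and aim an arrow at location markers.
; LeftShift triggers cooldown-gated character abilities such as boosts, slow motion or dissolve-teleport, several using cel-shader post-process blendables.
; Fast crashes eject and ragdoll non-Demon riders, and empty fuel disables the vehicle and shows WB_Win.
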(event OnComponentBeginOverlap(EnterBox)
  (params (OverlappedComponent :type Primitive%20Component%20Object%20Reference) (OtherActor :type Actor%20Object%20Reference) (OtherComp :type Primitive%20Component%20Object%20Reference) (OtherBodyIndex :type Integer) (bFromSweep :type Boolean) (SweepResult :type Hit%20Result%20Structure%20%28by%20ref%29))
  ;[1 1 1 1 66] Character Interactions / Movements
  (bind _asbp_character (Utilities|Casting|CastToBP_Character OtherActor))
  (Variables|/Game/Characters/BP_Character.BP_Character_C|SetInBox _asbp_character true)
  (bind _returnvalue (UserInterface|CreateWidget "/Game/Interfaces/Basbana.Basbana_C"))
  (UserInterface|Viewport|AddtoViewport _returnvalue 0))

(event OnComponentEndOverlap(EnterBox)
  (params (OverlappedComponent :type Primitive%20Component%20Object%20Reference) (OtherActor :type Actor%20Object%20Reference) (OtherComp :type Primitive%20Component%20Object%20Reference) (OtherBodyIndex :type Integer))
  ;[1 1 1 1 66] Character Interactions / Movements
  (bind _asbp_character (Utilities|Casting|CastToBP_Character OtherActor))
  (Variables|/Game/Characters/BP_Character.BP_Character_C|SetInBox _asbp_character false)
  (Widget|RemovefromParent (stale OnComponentBeginOverlap(EnterBox) _returnvalue)))

(event OnComponentEndOverlap(Box)
  (params (OverlappedComponent :type Primitive%20Component%20Object%20Reference) (OtherActor :type Actor%20Object%20Reference) (OtherComp :type Primitive%20Component%20Object%20Reference) (OtherBodyIndex :type Integer))
  ;[1 1 1 1 66] Character Interactions / Movements
  ;;[1 1 1] Character Crash Actions
  (Utilities|FlowControl|Delay 1e+01)
  (Utilities|FlowControl|DoOnce false) ; enters at Reset
)

(event OnComponentBeginOverlap(Box)
  (params (OverlappedComponent :type Primitive%20Component%20Object%20Reference) (OtherActor :type Actor%20Object%20Reference) (OtherComp :type Primitive%20Component%20Object%20Reference) (OtherBodyIndex :type Integer) (bFromSweep :type Boolean) (SweepResult :type Hit%20Result%20Structure%20%28by%20ref%29))
  ;[1 1 1 1 66] Character Interactions / Movements
  ;;[1 1 1] Character Crash Actions
  (Utilities|FlowControl|DoOnce false
    (:Completed
      (if (Variables|Default|GetInVehicle)
        (if (Variables|Default|GetIsDemon)
          (Development|PrintString "Yarram")
          (Rendering|SetVisibility (Variables|Default|GetFlame) true false)
          (elif (> (Class|WheeledVehicleMovementComponent|GetForwardSpeed (Variables|Default|GetVehicleComponent)) 7.5e+02)
            (CallFunction|OutOfVehicle)
            (bind _asbp_character (Utilities|Casting|CastToBP_Character (Game|Player|GetPlayerPawn 0)))
            (Default|Ragdoll _asbp_character)
            (else
              (Camera|PlayWorldCameraShake "/Game/Characters/MainCharacters/CameraShake/SetupCamShake.SetupCamShake_C" (Transformation|GetWorldLocation (Variables|Default|GetMoveMesh)) 0.0 1.5e+03))))))))

(event Custom|Fueller
  (bind _vehiclecomponent (Variables|Default|GetVehicleComponent))
  (bind _returnvalue (Class|WheeledVehicleMovementComponent|GetForwardSpeed _vehiclecomponent))
  (bind _returnvalue_2 (Math|Float|Truncate _returnvalue))
  (Utilities|Time|SetTimerbyEvent (delegate Custom|Fueller) 0.016667 true)
  (Utilities|IsValid (Game|GetPlayerCharacter 0)
    (:Is%20Not%20Valid
      (if (>= _returnvalue_2 0)
        (Variables|Default|SetFuel (- (Variables|Default|GetFuel) (/ (Math|Conversions|ToFloat(Integer) (+ _returnvalue_2 10)) 1e+04)))
        (if (<= (Variables|Default|GetFuel) 0.0)
          (Variables|Default|SetFuel 0.0)
          (Components|Activation|Deactivate (Variables|Default|GetVehicleComponent))
          ;[1 1 1 1 66] Character Interactions / Movements
          (Utilities|FlowControl|DoOnce false
            (:Completed
              (bind _returnvalue_3 (UserInterface|CreateWidget "/Game/Fuel/WB_Win.WB_Win_C"))
              (UserInterface|Viewport|AddtoViewport _returnvalue_3 0))))
        (else
          (Variables|Default|SetFuel (- (Variables|Default|GetFuel) (/ (Math|Conversions|ToFloat(Integer) (+ 0 10)) 2e+03)))
          (if (<= (Variables|Default|GetFuel) 0.0)
            (Variables|Default|SetFuel 0.0)
            (Components|Activation|Deactivate (Variables|Default|GetVehicleComponent))
            (Utilities|FlowControl|DoOnce false
              (:Completed
                (bind _returnvalue_4 (UserInterface|CreateWidget "/Game/Fuel/WB_Win.WB_Win_C"))
                (UserInterface|Viewport|AddtoViewport _returnvalue_4 0)))))))))

(event Custom|OutOfVehicle
  ;[1 1 1 1 66] Character Interactions / Movements
  (CallFunction|OutOfVehicleFunc)
  (CallFunction|PP (Variables|Default|GetPProcess) (stale Custom|GetInVehicle _returnvalue) 0.9)
  (Rendering|SetVisibility (Variables|Default|GetStaticMesh) false false)
  (CallFunction|DiasableMovement))

(event Custom|SteerRightRel
  ;[1 1 1 1 113] Scooter
  (Variables|Lean|SetPressinNow2 false)
  (Variables|Animations(forShow)|SetSteerDirection 0.0)
  (bind _rightlean (Timeline|RightLeanTime Reverse)
    (:Update
      (Transformation|SetRelativeRotation (Variables|Default|GetMoveMesh) (Math|Rotator|Lerp(Rotator) "0, 0, 0" (Variables|Animations(forShow)|GetEndRotationRight) _rightlean) false false)
      (Transformation|SetRelativeRotation (Variables|Default|GetSteer) (Math|Rotator|Lerp(Rotator) "0, 0, 0" (Variables|Animations(forShow)|GetSteerRotationRightEnd) _rightlean) false false))))

(event Custom|PP
  (params (Target :type Post%20Process%20Volume%20Object%20Reference) (InBlendableObject :type Blendable%20Interface%20Interface) (InWeight :type Float%20%28single-precision%29))
  (Rendering|AddorUpdateBlendable Target InBlendableObject InWeight :!class /Script/Engine.PostProcessVolume))

(event Custom|MakeUnVisible
  (bind _movemesh (Variables|Default|GetMoveMesh))
  (bind _dissolveflot (Timeline|Dissolving Play)
    (:Update
      (Rendering|Material|SetScalarParameterValueonMaterials _movemesh "Dissolve" _dissolveflot)
      (Rendering|Material|SetScalarParameterValueonMaterials _movemesh "Dissolve" _dissolveflot)
      (Rendering|Material|SetScalarParameterValueonMaterials (Variables|Default|GetCharacter) "Dissolve" _dissolveflot))))

(event Custom|MakeRevisible
  (bind _movemesh (Variables|Default|GetMoveMesh))
  (bind _dissolveflot (Timeline|Dissolving Reverse)
    (:Update
      (Rendering|Material|SetScalarParameterValueonMaterials _movemesh "Dissolve" _dissolveflot)
      (Rendering|Material|SetScalarParameterValueonMaterials _movemesh "Dissolve" _dissolveflot)
      (Rendering|Material|SetScalarParameterValueonMaterials (Variables|Default|GetCharacter) "Dissolve" _dissolveflot))))

(event Custom|DiasableMovement
  (bind _skeletalmesh (Variables|Default|GetSkeletalMesh))
  (bind _movemesh (Variables|Default|GetMoveMesh))
  (Class|PrimitiveComponent|SetConstraintMode _movemesh "XYPlane")
  (Class|PrimitiveComponent|SetConstraintMode _skeletalmesh "XYPlane")
  (Utilities|FlowControl|Delay 2.0)
  (Class|PrimitiveComponent|SetConstraintMode _skeletalmesh "SixDOF")
  (Class|PrimitiveComponent|SetConstraintMode _movemesh "SixDOF"))

(event Custom|GetInVehicle
  (params (InputMesh :type Skeletal%20Mesh%20Object%20Reference) (AnimInstance :type Object%20Class%20Reference) (Character :type Character%20Object%20Reference) (AnimInstanceAfterVehicle :type Object%20Class%20Reference) (IsSamurai :type Boolean) (IsGrandma :type Boolean) (IsWizard :type Boolean) (IsGamerGirl :type Boolean) (IsDemon :type Boolean) (IsGrandpa :type Boolean) (IsHomelessMan :type Boolean) (IsRichFemSci-Fi :type Boolean))
  ;[1 1 1 1 66] Character Interactions / Movements
  (Development|PrintString (Utilities|GetDisplayName Character))
  (Variables|Default|SetChar Character)
  (Utilities|WhichCharacter IsSamurai IsGrandma IsWizard IsGamerGirl IsDemon IsGrandpa IsHomelessMan IsRichFemSci-Fi)
  (Variables|Default|SetCharacterAnimClass AnimInstanceAfterVehicle)
  (Rendering|SetVisibility (Variables|Default|GetCharacter) true false)
  (CallFunction|ActivateMovement)
  (Variables|Default|SetInVehicle true)
  (Class|SkinnedMeshComponent|SetSkeletalMesh (Variables|Default|GetCharacter) InputMesh true)
  (Class|SkeletalMeshComponent|SetAnimClass (Variables|Default|GetCharacter) AnimInstance)
  (if (Variables|Default|GetIsWizard)
    (Transformation|SetRelativeLocation (Variables|Default|GetCharacter) "-0.500000,-37.179268,-10.000000" false false)
    (Rendering|SetVisibility (Variables|Default|GetStaticMesh) true false)
    (elif (Variables|Default|GetIsGrandma)
      (bind _returnvalue (Utilities|GrandmaDefaultView))
      (elif (Variables|Default|GetIsGamerGirl)
        (bind _returnvalue_2 (Rendering|Material|CreateDynamicMaterialInstance "/Game/CelShader/MobileCelShader/Presets/CelShaderMobileAnime.CelShaderMobileAnime" "None" "None" :!class /Script/Engine.KismetMaterialLibrary))
        (CallFunction|PP (Variables|Default|GetPProcess) _returnvalue_2 1.0)))))

(event Custom|ZeroFuel
  (bind _foundwidgets (Widget|GetAllWidgetsOfClass "/Game/Fuel/WB_Win.WB_Win_C" true))
  (Widget|RemovefromParent _foundwidgets)
  ;[1 1 1 1 66] Character Interactions / Movements
  (if (!= (Variables|Default|GetDolar2) 0)
    (Utilities|FlowControl|DoOnce false) ; enters at Reset
  ))

(event Custom|arrow2%20set%20directions
  (bind _arrow2 (Variables|Default|GetArrow2))
  (Utilities|Time|SetTimerbyEvent (delegate Custom|arrow2%20set%20directions) 0.033333 true)
  (bind _outactors (Actor|GetAllActorsOfClass "/Game/Map/LocationMarker/BP_LocationMarker.BP_LocationMarker_C"))
  (if (Utilities|Array|IsValidIndex _outactors)
    (bind _outactors_2 (Actor|GetAllActorsOfClass "/Game/Map/LocationMarker/BP_LocationMarker.BP_LocationMarker_C"))
    (for _array_element _outactors_2
      (Development|SetHiddeninGame _arrow2 false false)
      (Transformation|SetWorldRotation _arrow2 (Math|Rotator|FindLookatRotation (Transformation|GetWorldLocation _arrow2) (Transformation|GetActorLocation _array_element)) false false))
    (else
      (Development|SetHiddeninGame (Variables|Default|GetArrow2) true false))))

(event Custom|MySteer
  (params (Steering :type Float%20%28single-precision%29))
  ;[1 1 1 1 113] Scooter
  ;;[1 1 1] BaseControl
  (Class|WheeledVehicleMovementComponent|SetSteeringInput (Variables|Default|GetVehicleComponent) Steering))

(event Custom|MyThrottle
  (params (Throttle :type Float%20%28single-precision%29))
  (bind _vehiclecomponent (Variables|Default|GetVehicleComponent))
  ;[1 1 1 1 113] Scooter
  ;;[1 1 1] BaseControl
  (Class|WheeledVehicleMovementComponent|SetThrottleInput _vehiclecomponent Throttle)
  (Variables|Animations(forShow)|SetSpeed (Class|WheeledVehicleMovementComponent|GetForwardSpeed _vehiclecomponent)))

(event Custom|SteerLeftPres
  ;[1 1 1 1 113] Scooter
  (if (Variables|Lean|GetPressinNow2)
    (Development|PrintString "1Error" true true "(R=1.000000,G=0.000000,B=0.047369,A=1.000000)")
    (else
      (Variables|Lean|SetPressingNow true)
      (Variables|Animations(forShow)|SetSteerDirection -5e+01)
      (bind _leftlean (Timeline|LeftLeanTime Play)
        (:Update
          (Transformation|SetRelativeRotation (Variables|Default|GetMoveMesh) (Math|Rotator|Lerp(Rotator) "0, 0, 0" (Variables|Animations(forShow)|GetEndRotationLeft) _leftlean) false false)
          (Transformation|SetRelativeRotation (Variables|Default|GetSteer) (Math|Rotator|Lerp(Rotator) "0, 0, 0" (Variables|Animations(forShow)|GetSteerRotationLeftEnd) _leftlean) false false))))))

(event Custom|SteerLeftRel
  ;[1 1 1 1 113] Scooter
  (Variables|Lean|SetPressingNow false)
  (Variables|Animations(forShow)|SetSteerDirection 0.0)
  (bind _leftlean (Timeline|LeftLeanTime Reverse)
    (:Update
      (Transformation|SetRelativeRotation (Variables|Default|GetMoveMesh) (Math|Rotator|Lerp(Rotator) "0, 0, 0" (Variables|Animations(forShow)|GetEndRotationLeft) _leftlean) false false)
      (Transformation|SetRelativeRotation (Variables|Default|GetSteer) (Math|Rotator|Lerp(Rotator) "0, 0, 0" (Variables|Animations(forShow)|GetSteerRotationLeftEnd) _leftlean) false false))))

(event Custom|SteerRightPres
  ;[1 1 1 1 113] Scooter
  (if (Variables|Lean|GetPressingNow)
    (Development|PrintString "2Error" true true "(R=1.000000,G=0.000000,B=0.880068,A=1.000000)")
    (else
      (Variables|Lean|SetPressinNow2 true)
      (Variables|Animations(forShow)|SetSteerDirection 5e+01)
      (bind _rightlean (Timeline|RightLeanTime Play)
        (:Update
          (Transformation|SetRelativeRotation (Variables|Default|GetMoveMesh) (Math|Rotator|Lerp(Rotator) "0, 0, 0" (Variables|Animations(forShow)|GetEndRotationRight) _rightlean) false false)
          (Transformation|SetRelativeRotation (Variables|Default|GetSteer) (Math|Rotator|Lerp(Rotator) "0, 0, 0" (Variables|Animations(forShow)|GetSteerRotationRightEnd) _rightlean) false false))))))

(event EventBeginPlay
  (Utilities|FlowControl|Sequence
    (:then_0
      (bind _returnvalue (UserInterface|CreateWidget "/Game/Vehicles/Speed.Speed_C"))
      (UserInterface|Viewport|AddtoViewport _returnvalue 0)
      (CallFunction|Fueller))
    (:then_1
      (bind _outactors (Actor|GetAllActorsOfClass "/Game/Level_Database/BP_LevelDatabase.Bp_LevelDatabase_C"))
      (for _array_element _outactors
        (Variables|Default|SetDolar2 (Variables|/Game/Level_Database/BP_LevelDatabase.Bp_LevelDatabase_C|GetDolar _array_element))))
    (:then_2
      (CallFunction|Arrow2SetDirections))
    (:then_3
      (bind _outactors_2 (Actor|GetAllActorsOfClasswithTag "/Script/Engine.PostProcessVolume" "Samurai"))
      (for _array_element_2 _outactors_2
        (Variables|Default|SetPProcess _array_element_2)))))

(event Input|ActionEvents|InputActionSteerRight
  (params (Key :type Key%20Structure :default "None"))
  ;[1 1 1 1 113] Scooter
  (:Pressed
    (if (Variables|Lean|GetPressingNow)
      (Development|PrintString "2Error" true true "(R=1.000000,G=0.000000,B=0.880068,A=1.000000)")
      (else
        (Variables|Lean|SetPressinNow2 true)
        (Variables|Animations(forShow)|SetSteerDirection 5e+01)
        (bind _rightlean (Timeline|RightLeanTime Play)
          (:Update
            (Transformation|SetRelativeRotation (Variables|Default|GetMoveMesh) (Math|Rotator|Lerp(Rotator) "0, 0, 0" (Variables|Animations(forShow)|GetEndRotationRight) _rightlean) false false)
            (Transformation|SetRelativeRotation (Variables|Default|GetSteer) (Math|Rotator|Lerp(Rotator) "0, 0, 0" (Variables|Animations(forShow)|GetSteerRotationRightEnd) _rightlean) false false))))))
  (:Released
    (Variables|Lean|SetPressinNow2 false)
    (Variables|Animations(forShow)|SetSteerDirection 0.0)
    (Timeline|RightLeanTime Reverse)))

(event Input|ActionEvents|InputActionSteerLeft
  (params (Key :type Key%20Structure :default "None"))
  ;[1 1 1 1 113] Scooter
  (:Pressed
    (if (Variables|Lean|GetPressinNow2)
      (Development|PrintString "1Error" true true "(R=1.000000,G=0.000000,B=0.047369,A=1.000000)")
      (else
        (Variables|Lean|SetPressingNow true)
        (Variables|Animations(forShow)|SetSteerDirection -5e+01)
        (bind _leftlean (Timeline|LeftLeanTime Play)
          (:Update
            (Transformation|SetRelativeRotation (Variables|Default|GetMoveMesh) (Math|Rotator|Lerp(Rotator) "0, 0, 0" (Variables|Animations(forShow)|GetEndRotationLeft) _leftlean) false false)
            (Transformation|SetRelativeRotation (Variables|Default|GetSteer) (Math|Rotator|Lerp(Rotator) "0, 0, 0" (Variables|Animations(forShow)|GetSteerRotationLeftEnd) _leftlean) false false))))))
  (:Released
    (Variables|Lean|SetPressingNow false)
    (Variables|Animations(forShow)|SetSteerDirection 0.0)
    (Timeline|LeftLeanTime Reverse)))

(event Input|AxisEvents|InputAxisThrottle
  (params (AxisValue :type Float%20%28single-precision%29))
  (bind _particlesystem (Variables|Default|GetParticleSystem))
  ;[1 1 1 1 113] Scooter
  ;;[1 1 1] BaseControl
  (CallFunction|MyThrottle AxisValue)
  (if (> AxisValue 0.0)
    (Components|Activation|Deactivate _particlesystem)
    (else
      (Components|Activation|Activate _particlesystem false))))

(event Input|AxisEvents|InputAxisSteer
  (params (AxisValue :type Float%20%28single-precision%29))
  ;[1 1 1 1 113] Scooter
  ;;[1 1 1] BaseControl
  (CallFunction|MySteer AxisValue))

(event Input|KeyboardEvents|T
  (params (Key :type Key%20Structure :default "None"))
  ;[1 1 1 1 66] Character Interactions / Movements
  (:Pressed
    (CallFunction|OutOfVehicle)))

(event Input|KeyboardEvents|SpaceBar
  (params (Key :type Key%20Structure :default "None"))
  ;[1 1 1 1 113] Scooter
  (:Pressed
    (Transformation|Teleport (+ (Transformation|GetActorLocation) "0, 0,100.000000") (Math|Rotator|MakeRotator 0.0 0.0 (.yaw (Transformation|GetActorRotation))))))

(event Input|KeyboardEvents|LeftShift
  (params (Key :type Key%20Structure :default "None"))
  (:Pressed
    (if (Variables|Default|GetIsWizard)
      (Utilities|Wizard)
      (elif (Variables|Default|GetIsSamurai)
        (Utilities|Samurai)
        (elif (Variables|Default|GetIsGrandma)
          (Utilities|Grandma (stale Custom|GetInVehicle _returnvalue))
          (elif (Variables|Default|GetIsGrandpa)
            (Utilities|Grandpa)
            (elif (Variables|Default|GetIsRichFemSci-Fi)
              (Utilities|RichFemSci-Fi))))))))

(event Input|KeyboardEvents|1
  (params (Key :type Key%20Structure :default "None")))

(fn ConstructionScript
  (|CallParentFunction))

(fn ActivateMovement
  (Class|PrimitiveComponent|SetConstraintMode (Variables|Default|GetMoveMesh) "None")
  (Class|PrimitiveComponent|SetConstraintMode (Variables|Default|GetSkeletalMesh) "None"))

(fn OutOfVehicleFunc
  (CallFunction|ActivateMovement)
  (Variables|Default|SetInVehicle false)
  (bind _outactors (Actor|GetAllActorsOfClass "/Game/Characters/BP_Character.BP_Character_C"))
  (for _array_element _outactors
    (Rendering|SetVisibility (Variables|/Script/Engine.Character|GetMesh _array_element) true false)
    (Collision|SetActorEnableCollision _array_element true)
    (Transformation|Teleport _array_element (Transformation|GetWorldLocation (Variables|Default|GetOutOf)) "0, 0, 0")
    (Utilities|IsValid _array_element
      (:Is%20Valid
        (Pawn|Possess (Game|GetPlayerController 0) _array_element)
        (Class|SkinnedMeshComponent|SetSkeletalMesh (Variables|Default|GetCharacter) 0 true)))))