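; Police car vehicle Blueprint that turns player axis input into driving through a SimpleWheeledVehicleMovement component.
; Steer sets the angle of wheels 0 and 1, and Throttle applies drive torque to wheels 2 and 3.
; Brake applies brake torque to wheel 1 only, with each input scaled by a fixed multiplier.
; The construction script only calls its parent.
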(event Input|AxisEvents|InputAxisSteer
  (params (AxisValue :type Float%20%28single-precision%29))
  (bind _returnvalue (* AxisValue 45.0))
  (bind _simplewheeledvehiclemovement (Variables|Default|GetSimpleWheeledVehicleMovement))
  ;[1 1 1] BaseControl
  (Class|SimpleWheeledVehicleMovementComponent|SetSteerAngle _simplewheeledvehiclemovement _returnvalue)
  (Class|SimpleWheeledVehicleMovementComponent|SetSteerAngle _simplewheeledvehiclemovement _returnvalue 1))

(event Input|AxisEvents|InputAxisThrottle
  (params (AxisValue :type Float%20%28single-precision%29))
  (bind _returnvalue (* AxisValue 1.5e+03))
  (bind _simplewheeledvehiclemovement (Variables|Default|GetSimpleWheeledVehicleMovement))
  ;[1 1 1] BaseControl
  (Class|SimpleWheeledVehicleMovementComponent|SetDriveTorque _simplewheeledvehiclemovement _returnvalue 2)
  (Class|SimpleWheeledVehicleMovementComponent|SetDriveTorque _simplewheeledvehiclemovement _returnvalue 3))

(event Input|AxisEvents|InputAxisBrake
  (params (AxisValue :type Float%20%28single-precision%29))
  ;[1 1 1] BaseControl
  (Class|SimpleWheeledVehicleMovementComponent|SetBrakeTorque (Variables|Default|GetSimpleWheeledVehicleMovement) (* AxisValue 5e+02) 1))

(fn ConstructionScript
  (|CallParentFunction))