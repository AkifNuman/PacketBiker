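; BP_Fuel drains a Fuel value according to the speed shown in the Speed widget.
; On BeginPlay it caches the top-level Speed widget and starts Fueller, which re-arms itself on a looping 60 Hz timer.
; While no valid player character exists, each tick subtracts an amount scaled from SpeedInt plus a base offset.
; Fuel exactly equal to zero sets the widget's SpeedInt to zero.
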(event Custom|Fueller
  (Utilities|Time|SetTimerbyEvent (delegate Custom|Fueller) 0.016667 true)
  (Utilities|IsValid (Game|GetPlayerCharacter 0)
    (:Is%20Not%20Valid
      (Variables|Default|SetFuel (- (Variables|Default|GetFuel) (/ (Math|Conversions|ToFloat(Integer) (+ (Variables|/Game/Vehicles/Speed.Speed_C|GetSpeedInt (Variables|Default|GetSpeedBp)) 10)) 1e+03)))
      (if (== (Variables|Default|GetFuel) 0.0)
        (Variables|/Game/Vehicles/Speed.Speed_C|SetSpeedInt (Variables|Default|GetSpeedBp) 0)))))

(event EventBeginPlay
  (bind _foundwidgets (Widget|GetAllWidgetsOfClass "/Game/Vehicles/Speed.Speed_C" true))
  (for _array_element _foundwidgets
    (Variables|Default|SetSpeedBp _array_element)
    (CallFunction|Fueller)))

(fn ConstructionScript)