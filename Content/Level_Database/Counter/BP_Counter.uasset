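; Mission countdown actor that shows the counter widgets and penalizes the player when time runs out.
; IsMissionComplete re-fires itself on a fast looping timer, with a one-second Delay pacing each MissionCounter decrement.
; At zero, if a BP_TargetCalculator exists, it deducts Dolar from Bp_LevelDatabase.
; Nested GetAllActorsOfClass loops then destroy markers and calculators, remove widgets, hide target and restaurant points, and destroy the counter.
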(event Custom|Is%20Mission%20Complete
  (Utilities|Time|SetTimerbyEvent (delegate Custom|Is%20Mission%20Complete) 0.033333 true)
  (Utilities|FlowControl|Delay 1.0)
  (bind _output_get (Variables|Default|SetMissionCounter (- (Variables|Default|GetMissionCounter) 1)))
  (Development|PrintString (Utilities|String|ToString(Integer) _output_get))
  (if (== (Variables|Default|GetMissionCounter) 0)
    (bind _outactors (Actor|GetAllActorsOfClass "/Game/Mission/BP_TargetCalculator.BP_TargetCalculator_C"))
    (if (Utilities|Array|IsValidIndex _outactors)
      (bind _outactors_2 (Actor|GetAllActorsOfClass "/Game/Level_Database/BP_LevelDatabase.Bp_LevelDatabase_C"))
      (for _array_element _outactors_2
        (Development|PrintString "Hello1")
        (bind _output_get_2 (Variables|/Game/Level_Database/BP_LevelDatabase.Bp_LevelDatabase_C|SetDolar _array_element (- (Variables|/Game/Level_Database/BP_LevelDatabase.Bp_LevelDatabase_C|GetDolar _array_element) 5)))
        (Development|PrintString (Utilities|String|Append "dolar" (Utilities|String|ToString(Integer) _output_get_2)))
        (bind _outactors_3 (Actor|GetAllActorsOfClass "/Game/Map/LocationMarker/BP_LocationMarkerRes.BP_LocationMarkerRes_C"))
        (for _array_element_2 _outactors_3
          (Actor|DestroyActor _array_element_2)
          (bind _outactors_4 (Actor|GetAllActorsOfClass "/Game/Mission/BP_TargetCalculator.BP_TargetCalculator_C"))
          (for _array_element_3 _outactors_4
            (Actor|DestroyActor _array_element_3)
            (bind _foundwidgets (Widget|GetAllWidgetsOfClass "/Game/Level_Database/WB_MissionCounter.WB_MissionCounter_C" true))
            (for _array_element_4 _foundwidgets
              (Widget|RemovefromParent _array_element_4)
              (bind _outactors_5 (Actor|GetAllActorsOfClass "/Game/Mission/BP_TargetPoint.BP_TargetPoint_C"))
              (for _array_element_5 _outactors_5
                (Rendering|SetActorHiddenInGame _array_element_5 true)
                (bind _outactors_6 (Actor|GetAllActorsOfClass "/Game/Mission/BP_RestaurantPoint.BP_RestaurantPoint_C"))
                (for _array_element_6 _outactors_6
                  (Rendering|SetActorHiddenInGame _array_element_6 true)
                  (Widget|RemovefromParent (stale EventBeginPlay _returnvalue_2))
                  (Actor|DestroyActor)))))))
      (else
        (Development|PrintString "Hello")))))

(event EventBeginPlay
  (Utilities|FlowControl|Sequence
    (:then_0
      (CallFunction|IsMissionComplete))
    (:then_1
      (bind _returnvalue (UserInterface|CreateWidget "/Game/Level_Database/WB_MissionCounter.WB_MissionCounter_C" (Game|GetPlayerController 0)))
      (UserInterface|Viewport|AddtoViewport _returnvalue 0))
    (:then_2
      (bind _returnvalue_2 (UserInterface|CreateWidget "/Game/Level_Database/Counter/WB_Counter.WB_Counter_C"))
      (UserInterface|Viewport|AddtoViewport _returnvalue_2 0))))

(event Collision|EventActorBeginOverlap
  (params (OtherActor :type Actor%20Object%20Reference)))

(fn ConstructionScript)