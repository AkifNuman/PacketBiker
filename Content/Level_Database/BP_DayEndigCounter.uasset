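; BP_DayEndigCounter is an actor that counts elapsed time to end in-game days and show the day-ending screen.
; Tick feeds a one-second Delay, acting as a repeating timer that increments DayEndCounter.
; At each multiple of ten it prints a debug string, increments DayCounter, removes all widgets, pauses the game and adds a new WB_DayEnding widget to the viewport.
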(event EventBeginPlay)

(event Collision|EventActorBeginOverlap
  (params (OtherActor :type Actor%20Object%20Reference)))

(event EventTick
  (params (DeltaSeconds :type Float%20%28single-precision%29))
  (Utilities|FlowControl|Delay 1.0)
  (Variables|Default|SetDayEndCounter (+ (Variables|Default|GetDayEndCounter) 1))
  (if (== (Math|Integer|%(Integer) (Variables|Default|GetDayEndCounter) 10) 0)
    (Development|PrintString "Hello")
    (Variables|Default|SetDayCounter (+ (Variables|Default|GetDayCounter) 1))
    (Viewport|RemoveAllWidgets)
    (Game|SetGamePaused true)
    (bind _returnvalue (UserInterface|CreateWidget "/Game/Level_Database/WB_DayEnding.WB_DayEnding_C" (Game|GetPlayerController 0)))
    (UserInterface|Viewport|AddtoViewport _returnvalue 0)))

(fn ConstructionScript)