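; BP_HomelessMan is a homeless-man character Blueprint that lets the player board a scooter with the F key.
; Pressing F calls ScooterGetSamWar, which, while InBox is true, loops over every Scooter_BP rather than picking one.
; Each iteration hides the character mesh, passes the hobo mesh and animation class to GetInVehicle with IsSamurai set, and possesses that scooter.
; It also disables the character's collision and adds fuel bar and scooter interface widgets.
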(event EventBeginPlay
  (|CallParentFunction) ; This node is disabled and will not be called.\nDrag off pins to build functionality.
)

(event Collision|EventActorBeginOverlap
  (params (OtherActor :type Actor%20Object%20Reference)))

(event EventTick
  (params (DeltaSeconds :type Float%20%28single-precision%29))
  (|CallParentFunction DeltaSeconds) ; This node is disabled and will not be called.\nDrag off pins to build functionality.
)

(event Input|KeyboardEvents|F
  (params (Key :type Key%20Structure))
  (:Pressed
    (CallFunction|ScooterGetSamWar)))

(fn ConstructionScript
  (|CallParentFunction))

(fn ScooterGetSamWar
  (if (Variables|Default|GetInBox)
    (bind _outactors (Actor|GetAllActorsOfClass "/Game/Vehicles/Motorcycles/Scooter/Scooter_BP.Scooter_BP_C"))
    (for _array_element _outactors
      (Variables|/Game/Vehicles/Motorcycles/Scooter/Scooter_BP.Scooter_BP_C|SetInVehicle _array_element true)
      (bind _asbp_homeless_man (Utilities|Casting|CastToBP_HomelessMan (Game|Player|GetPlayerPawn 0)))
      (Rendering|SetVisibility (Variables|Character|GetMesh) false false)
      (Default|GetinVehicle _array_element "/Game/PolygonCityChar/Characters/SK_Character_Hobo.SK_Character_Hobo" "/Game/Characters/MainCharacters/Animations/fCityCharsChars/CityCharacterAnimBP.CityCharacterAnimBP_C" _asbp_homeless_man 0 true false false false false false false false)
      (Pawn|Possess (Game|GetPlayerController 0) _array_element)
      (Variables|Default|SetInBoxPressed false)
      (Collision|SetActorEnableCollision false)
      (bind _returnvalue (UserInterface|CreateWidget "/Game/Fuel/WB_FuelBar.WB_FuelBar_C"))
      (UserInterface|Viewport|AddtoViewport _returnvalue 0)
      (bind _returnvalue_2 (UserInterface|CreateWidget "/Game/Interfaces/ScooterInterface.ScooterInterface_C"))
      (UserInterface|Viewport|AddtoViewport _returnvalue_2 0))))