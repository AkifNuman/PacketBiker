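; Dash collectable pickup that spins in place and adds to a dash collectable count kept in Bp_LevelDatabase.
; Tick turns it by a fixed yaw step each frame and uses a Delay as a seconds counter, destroying it after about 30 seconds.
; Box overlap increments and prints the count on database actors, then destroys the pickup.
; That overlap logic runs only when player character 0 is invalid, and never checks the overlapping actor.
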(event OnComponentBeginOverlap(Box)
  (params (OverlappedComponent :type Primitive%20Component%20Object%20Reference) (OtherActor :type Actor%20Object%20Reference) (OtherComp :type Primitive%20Component%20Object%20Reference) (OtherBodyIndex :type Integer) (bFromSweep :type Boolean) (SweepResult :type Hit%20Result%20Structure%20%28by%20ref%29))
  (Utilities|IsValid (Game|GetPlayerCharacter 0)
    (:Is%20Not%20Valid
      (bind _outactors (Actor|GetAllActorsOfClass "/Game/Level_Database/BP_LevelDatabase.Bp_LevelDatabase_C"))
      (for _array_element _outactors
        (bind _output_get (Variables|/Game/Level_Database/BP_LevelDatabase.Bp_LevelDatabase_C|SetDashCollectableCount _array_element (+ (Variables|/Game/Level_Database/BP_LevelDatabase.Bp_LevelDatabase_C|GetDashCollectableCount _array_element) 1)))
        (Development|PrintString (Utilities|String|ToString(Integer) _output_get))
        (Actor|DestroyActor)))))

(event EventBeginPlay)

(event Collision|EventActorBeginOverlap
  (params (OtherActor :type Actor%20Object%20Reference)))

(event EventTick
  (params (DeltaSeconds :type Float%20%28single-precision%29))
  (bind _returnvalue (Transformation|GetActorRotation))
  (Transformation|SetActorRotation (Math|Rotator|MakeRotator (.roll _returnvalue) (.pitch _returnvalue) (+ (.yaw _returnvalue) 1.0)))
  (Utilities|FlowControl|Delay 1.0)
  (Variables|Default|SetTime (+ (Variables|Default|GetTime) 1))
  (if (>= (Variables|Default|GetTime) 30)
    (Actor|DestroyActor)))

(fn ConstructionScript)