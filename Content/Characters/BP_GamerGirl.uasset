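; BP_GamerGirl is a playable character Blueprint for a gamer girl who can ride scooters.
; The SpecialForce input toggles her post-process effect on and off through a FlipFlop.
; Pressing F while InBox loops over all Scooter_BP actors, passing her mesh, animation class and an anime post-process flag to GetInVehicle.
; The player controller then possesses the scooter and the character destroys itself.
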(event Input|ActionEvents|InputActionSpecialForce
  (params (Key :type Key%20Structure :default "None"))
  (bind _postprocess (Variables|Default|GetPostProcess))
  (:Pressed
    (Utilities|FlowControl|FlipFlop
      (:A
        (Rendering|SetVisibility _postprocess true false))
      (:B
        (Rendering|SetVisibility _postprocess false false)))))

(event Input|KeyboardEvents|F
  (params (Key :type Key%20Structure :default "None"))
  (:Pressed
    (CallFunction|ScooterGetGamerGirl)))

(fn ConstructionScript
  (|CallParentFunction))

(fn ScooterGetGamerGirl
  (if (Variables|Default|GetInBox)
    (bind _outactors (Actor|GetAllActorsOfClass "/Game/Vehicles/Motorcycles/Scooter/Scooter_BP.Scooter_BP_C"))
    (for _array_element _outactors
      (Rendering|SetVisibility (Variables|Character|GetMesh) false false)
      (Variables|Default|SetInBoxPressed true)
      (Default|GetinVehicle _array_element "/Game/PolygonCityChar/Characters/SK_Character_GamerGirl.SK_Character_GamerGirl" "/Game/Characters/MainCharacters/Animations/fCityCharsChars/CityCharacterAnimBP.CityCharacterAnimBP_C" true self)
      (Pawn|Possess (Game|GetPlayerController 0) _array_element)
      (Actor|DestroyActor)
      (Variables|Default|SetInBoxPressed false))))