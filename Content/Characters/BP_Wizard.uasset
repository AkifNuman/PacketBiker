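; BP_Wizard is a wizard character that can mount a scooter and switch to ragdoll physics.
; Pressing F while InBox is set loops over every Scooter_BP, hides the wizard mesh, passes wizard mesh and animation classes to GetInVehicle, disables collision and possesses the scooter.
; The loop does not pick a specific scooter, so each one receives the call and possession in turn.
; A separate function enables physics simulation on the mesh for ragdolling.
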(event Input|KeyboardEvents|F
  (params (Key :type Key%20Structure))
  (:Pressed
    (CallFunction|ScooterGetWizard)))

(fn ConstructionScript
  (|CallParentFunction))

(fn ScooterGetWizard
  (if (Variables|Default|GetInBox)
    (bind _outactors (Actor|GetAllActorsOfClass "/Game/Vehicles/Motorcycles/Scooter/Scooter_BP.Scooter_BP_C"))
    (for _array_element _outactors
      (Rendering|SetVisibility (Variables|Character|GetMesh) false false)
      (Variables|Default|SetInBoxPressed true)
      (bind _asbp_wizard (Utilities|Casting|CastToBP_Wizard (Game|Player|GetPlayerPawn 0)))
      (Default|GetinVehicle _array_element "/Game/PolygonFantasyCharacters/Characters/SK_Character_Male_Wizard.SK_Character_Male_Wizard" "/Game/Characters/MainCharacters/Animations/fFantasyChars/FantasyCharacterAnimBP.FantasyCharacterAnimBP_C" _asbp_wizard false false true false "/Game/Characters/MainCharacters/Animations/fFantasyChars/JustChar/FantasyCharsMovementAnimBP.FantasyCharsMovementAnimBP_C")
      (Collision|SetActorEnableCollision false)
      (Pawn|Possess (Game|GetPlayerController 0) _array_element)
      (Variables|Default|SetInBoxPressed false))))

(fn RagdollWizard
  (Physics|SetSimulatePhysics (Variables|Character|GetMesh) true))