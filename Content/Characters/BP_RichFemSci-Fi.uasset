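; BP_RichFemSci-Fi is a rich female sci-fi character that can board a scooter when F is pressed.
; If InBox is set, it loops over every Scooter_BP, hides its mesh and passes its skeletal mesh, anim Blueprint and itself to GetInVehicle.
; Player 0's controller then possesses that scooter and the character is destroyed, with no filtering for the nearby scooter.
; A separate function ragdolls the mesh by enabling physics simulation.
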(event Input|KeyboardEvents|F
  (params (Key :type Key%20Structure))
  (:Pressed
    (CallFunction|ScooterGetRichFemSci-Fi)))

(fn ConstructionScript
  (|CallParentFunction))

(fn ScooterGetRichFemSci-Fi
  (if (Variables|Default|GetInBox)
    (bind _outactors (Actor|GetAllActorsOfClass "/Game/Vehicles/Motorcycles/Scooter/Scooter_BP.Scooter_BP_C"))
    (for _array_element _outactors
      (Rendering|SetVisibility (Variables|Character|GetMesh) false false)
      (Variables|Default|SetInBoxPressed true)
      (Default|GetinVehicle _array_element "/Game/PolygonScifi/Meshes/Characters/SK_Character_Rich_Female_01.SK_Character_Rich_Female_01" "/Game/Characters/MainCharacters/Animations/fSci-fiChars/Sci-FI-CharacterAnimBP.Sci-FI-CharacterAnimBP_C" false self)
      (Pawn|Possess (Game|GetPlayerController 0) _array_element)
      (Actor|DestroyActor)
      (Variables|Default|SetInBoxPressed false))))

(fn RagdollRichFemSci-Fi
  (Physics|SetSimulatePhysics (Variables|Character|GetMesh) true))