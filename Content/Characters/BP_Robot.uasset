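; BP_Robot is a robot character that can board a scooter when F is pressed while InBox is true.
; It loops over every Scooter_BP actor, hides the robot mesh, passes its mesh and animation classes to GetInVehicle with the samurai flag set, and possesses the scooter.
; The same loop disables the robot's collision and adds fuel bar and scooter interface widgets to the viewport.
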(event EventBeginPlay
  (|CallParentFunction) ; This node is disabled and will not be called.\nDrag off pins to build functionality.
)

(event Collision|EventActorBeginOverlap
  (params (OtherActor :type Actor%20Object%20Reference)))

(event EventTick
  (params (DeltaSeconds :type Float%20%28single-precision%29))
  (|CallParentFunction DeltaSeconds) ; This node is disabled and will not be called.\nDrag off pins to build functionality.
)

(event Input|KeyboardEvents|F
  (params (Key :type Key%20Structure :default "None"))
  (:Pressed
    (CallFunction|ScooterGetSamWar)))

(fn ConstructionScript
  (|CallParentFunction))

(fn ScooterGetSamWar
  (if (Variables|Default|GetInBox)
    (bind _outactors (Actor|GetAllActorsOfClass "/Game/Vehicles/Motorcycles/Scooter/Scooter_BP.Scooter_BP_C"))
    (for _array_element _outactors
      (Variables|/Game/Vehicles/Motorcycles/Scooter/Scooter_BP.Scooter_BP_C|SetInVehicle _array_element true)
      (bind _asbp_robot (Utilities|Casting|CastToBP_Robot (Game|Player|GetPlayerPawn 0)))
      (Rendering|SetVisibility (Variables|Character|GetMesh) false false)
      (Default|GetinVehicle _array_element "/Game/PolygonScifi/Meshes/Characters/SK_Character_Robot_01.SK_Character_Robot_01" "/Game/Characters/MainCharacters/Animations/fSci-fiChars/Sci-FI-CharacterAnimBP.Sci-FI-CharacterAnimBP_C" _asbp_robot "/Game/Characters/MainCharacters/Animations/fSci-fiChars/JustChar/Sci-Fi-CharsMovementAnimBP.Sci-Fi-CharsMovementAnimBP_C" true false false false false false false false)
      (Pawn|Possess (Game|GetPlayerController 0) _array_element)
      (Variables|Default|SetInBoxPressed false)
      (Collision|SetActorEnableCollision false)
      (bind _returnvalue (UserInterface|CreateWidget "/Game/Fuel/WB_FuelBar.WB_FuelBar_C"))
      (UserInterface|Viewport|AddtoViewport _returnvalue 0)
      (bind _returnvalue_2 (UserInterface|CreateWidget "/Game/Interfaces/ScooterInterface.ScooterInterface_C"))
      (UserInterface|Viewport|AddtoViewport _returnvalue_2 0))))