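; BP_Demon is the Red Demon character, which can mount a scooter and take control of it.
; Pressing F while InBox is true hides the demon's mesh, passes its skeletal mesh and anim classes to GetInVehicle, possesses the scooter and disables its own collision.
; This loop runs over every Scooter_BP in the level, adding fuel bar and scooter widgets each time.
; A separate function ragdolls the mesh by enabling physics simulation.
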(event EventBeginPlay)

(event Collision|EventActorBeginOverlap
  (params (OtherActor :type Actor%20Object%20Reference)))

(event EventTick
  (params (DeltaSeconds :type Float%20%28single-precision%29)))

(event Input|KeyboardEvents|F
  (params (Key :type Key%20Structure))
  (:Pressed
    (CallFunction|ScooterGetRedDemon)))

(fn ConstructionScript
  (|CallParentFunction))

(fn ScooterGetRedDemon
  (if (Variables|Default|GetInBox)
    (bind _outactors (Actor|GetAllActorsOfClass "/Game/Vehicles/Motorcycles/Scooter/Scooter_BP.Scooter_BP_C"))
    (for _array_element _outactors
      (Rendering|SetVisibility (Variables|Character|GetMesh) false false)
      (Variables|Default|SetInBoxPressed true)
      (Default|GetinVehicle _array_element "/Game/PolygonFantasyRivals/Meshes/Characters/SK_BR_Character_RedDemon_01.SK_BR_Character_RedDemon_01" "/Game/Characters/MainCharacters/Animations/fRivalsChars/RivalsCharacterAnimBP1.RivalsCharacterAnimBP1_C" self "/Game/Characters/MainCharacters/Animations/fRivalsChars/JustChar/RivalsCharMovementAnimBP1.RivalsCharMovementAnimBP1_C" false false false false true false false false)
      (Pawn|Possess (Game|GetPlayerController 0) _array_element)
      (Variables|Default|SetInBoxPressed false)
      (Collision|SetActorEnableCollision false)
      (bind _returnvalue (UserInterface|CreateWidget "/Game/Fuel/WB_FuelBar.WB_FuelBar_C"))
      (UserInterface|Viewport|AddtoViewport _returnvalue 0)
      (bind _returnvalue_2 (UserInterface|CreateWidget "/Game/Interfaces/ScooterInterface.ScooterInterface_C"))
      (UserInterface|Viewport|AddtoViewport _returnvalue_2 0))))

(fn RagdollRedDemon
  (Physics|SetSimulatePhysics (Variables|Character|GetMesh) true))