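; BP_Grandpa is the Grandpa character, with a rechargeable slow-time ability and scooter boarding.
; A self-restarting timer and Delay count up to 60 seconds to arm the ability; R then slows the world for five seconds while speeding Grandpa up.
; F, when InBox is set, hides Grandpa, disables his collision, passes his mesh and animation classes to Scooter_BP, possesses it and adds fuel and scooter widgets.
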(event Custom|TimeStop
  (Utilities|Time|SetTimerbyEvent (delegate Custom|TimeStop) 0.033333)
  (Utilities|FlowControl|Delay 1.0)
  (bind _output_get (Variables|Default|SetTime (+ (Variables|Default|GetTime) 1)))
  (if (>= _output_get 60)
    (Variables|Default|SetisTimeStop true)))

(event EventBeginPlay
  (|CallParentFunction)
  (CallFunction|TimeStop))

(event Input|KeyboardEvents|F
  (params (Key :type Key%20Structure))
  (:Pressed
    (CallFunction|ScooterGetSamWar)))

(event Input|KeyboardEvents|R
  (params (Key :type Key%20Structure))
  (:Pressed
    (if (Variables|Default|GetisTimeStop)
      (Utilities|Time|SetGlobalTimeDilation 0.3)
      (Variables|Default|SetCustomTimeDilation 4.0)
      (Variables|Default|SetisTimeStop false)
      (Utilities|FlowControl|Delay 5.0)
      (Utilities|Time|SetGlobalTimeDilation 1.0)
      (Variables|Default|SetCustomTimeDilation 1.0)
      (Variables|Default|SetTime 0))))

(fn ConstructionScript
  (|CallParentFunction))

(fn ScooterGetSamWar
  (if (Variables|Default|GetInBox)
    (bind _outactors (Actor|GetAllActorsOfClass "/Game/Vehicles/Motorcycles/Scooter/Scooter_BP.Scooter_BP_C"))
    (for _array_element _outactors
      (Variables|/Game/Vehicles/Motorcycles/Scooter/Scooter_BP.Scooter_BP_C|SetInVehicle _array_element true)
      (bind _asbp_grandpa (Utilities|Casting|CastToBP_Grandpa (Game|Player|GetPlayerPawn 0)))
      (Rendering|SetVisibility (Variables|Character|GetMesh) false false)
      (Default|GetinVehicle _array_element "/Game/PolygonCityChar/Characters/SK_Character_Grandpa.SK_Character_Grandpa" "/Game/Characters/MainCharacters/Animations/fCityCharsChars/CityCharacterAnimBP.CityCharacterAnimBP_C" _asbp_grandpa "/Game/Characters/MainCharacters/Animations/fCityCharsChars/JustChar/CityCharMovementAnimBP.CityCharMovementAnimBP_C" false false false false false true false false)
      (Pawn|Possess (Game|GetPlayerController 0) _array_element)
      (Variables|Default|SetInBoxPressed false)
      (Collision|SetActorEnableCollision false)
      (bind _returnvalue (UserInterface|CreateWidget "/Game/Fuel/WB_FuelBar.WB_FuelBar_C"))
      (UserInterface|Viewport|AddtoViewport _returnvalue 0)
      (bind _returnvalue_2 (UserInterface|CreateWidget "/Game/Interfaces/ScooterInterface.ScooterInterface_C"))
      (UserInterface|Viewport|AddtoViewport _returnvalue_2 0))))